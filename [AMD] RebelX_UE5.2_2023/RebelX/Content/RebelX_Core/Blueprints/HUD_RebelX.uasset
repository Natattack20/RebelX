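; RebelX player HUD that creates and manages the core HUD, crosshair and notification widgets.
; On BeginPlay it casts the controlled pawn to Player_RebelX, passing its health component and reference into the widgets.
; Events forward crosshair prompts, hit markers, objective text and show/hide calls to those widgets.
; Notifications use a duplicate-filtered queue, played one at a time with sound and advanced by the widget's completion callback.
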(event `/Game/RebelX_Core/Blueprints/Interfaces/BPI_HUD.HideAllUI`
  (`Widget.SetVisibility` (`self.HUDCore`) "Hidden")
  (`Widget.SetVisibility` (`self.Crosshair`) "Hidden"))

(event `/Game/RebelX_Core/Blueprints/Interfaces/BPI_HUD.ShowAllUI`
  (`Widget.SetVisibility` (`self.HUDCore`) "Visible")
  (`Widget.SetVisibility` (`self.Crosshair`) "Visible"))

(event `self.ReceiveBeginPlay`
  ;[1 1 1] Get player reference
  (bind _asplayer_rebel_x (cast `/Game/RebelX_Core/Blueprints/Player_RebelX` (`Controller.K2_GetPawn` (`self.GetOwningPlayerController`)))
    (:`then`
      (set `self.PlayerReference` _asplayer_rebel_x)
      (`|ExecutionSequence`
        (:`then_0`
          (`|ExecutionSequence`
            (:`then_0`
              ;[1 1 1] Create HUD
              (bind _returnvalue (`|CreateWidget` "/Game/RebelX_Core/UserInterface/HUDCore.HUDCore_C" (`self.GetOwningPlayerController`) (`/Game/RebelX_Core/Blueprints/Player_RebelX.BP_Health` (`self.PlayerReference`))))
              (bind _output_get (set `self.HUDCore` _returnvalue))
              (`UserWidget.AddToPlayerScreen` _output_get 0))
            (:`then_1`
              ;[1 1 1] Create crosshair
              (bind _returnvalue_2 (`|CreateWidget` "/Game/RebelX_Core/UserInterface/WC_Crosshair.WC_Crosshair_C" (`self.GetOwningPlayerController`) (`self.PlayerReference`)))
              (bind _output_get_2 (set `self.Crosshair` _returnvalue_2))
              (`UserWidget.AddToPlayerScreen` _output_get_2 0))))
        (:`then_1`
          ;[1 1 1] Create HUD Notification
          (bind _returnvalue_3 (`|CreateWidget` "/Game/RebelX_Core/UserInterface/W_HUDNotification.W_HUDNotification_C" (`self.GetOwningPlayerController`) "Notification!"))
          (bind _output_get_3 (set `self.HUDNotification` _returnvalue_3))
          (`UserWidget.AddToViewport` _output_get_3 0)
          (`Widget.SetVisibility` _output_get_3 "Hidden")
          (add `/Game/RebelX_Core/UserInterface/W_HUDNotification.NotificationComplete` _output_get_3 (delegate `NotificationComplete`)))))
    (:`CastFailed`
      (`/Game/RebelX_Core/Blueprints/Functions/BP_DebugFunctions.DebugLog` "Cast to player charachter failed" "NewEnumerator2"))))

(event `/Game/RebelX_Core/Blueprints/Interfaces/BPI_HUD.ShowHitMark`
  ;[1 1 1] Show Hit Marker
  (`/Game/RebelX_Core/UserInterface/HUDCore.HitMarker` (`self.HUDCore`)))

(event `/Game/RebelX_Core/Blueprints/Interfaces/BPI_HUD.ShowCrosshairPrompt`
  (params (Prompt :type Text) (Type :type "/Game/RebelX_Core/Blueprints/Enums/E_CrosshairPromptTpye Enum" :default "NewEnumerator0") (Duration :type "Float (double-precision)") (KeepCrosshair :type Boolean) (IconBrush :type "SlateBrush Structure"))
  ;[1 1 1] Show Crosshair Prompt
  (`/Game/RebelX_Core/UserInterface/WC_Crosshair.ShowMessage` (`self.Crosshair`) Prompt Type Duration KeepCrosshair IconBrush))

(event `/Game/RebelX_Core/Blueprints/Interfaces/BPI_HUD.SetCrosshair`
  ;[1 1 1] Create crosshair
)

(event `/Game/RebelX_Core/Blueprints/Interfaces/BPI_HUD.HideCrosshairPrompt`
  ;[1 1 1] Show Crosshair Prompt
  (`/Game/RebelX_Core/UserInterface/WC_Crosshair.HideMessage` (`self.Crosshair`)))

(event `/Game/RebelX_Core/Blueprints/Interfaces/BPI_HUD.StopReloadWarning`
  ;[1 1 1] Reloading
)

(event `NotificationComplete`
  (bind _notificationque (`self.NotificationQue`))
  ;[1 1 1] Notification Complete
  (`KismetSystemLibrary.DelayUntilNextTick`) ; Wait until next tick before showing another notificaiton
  (`KismetArrayLibrary.Array_Remove` _notificationque)
  (if (`KismetArrayLibrary.Array_IsValidIndex` _notificationque)
    (`self.ShowNotification`)
    (else
      (`Widget.SetVisibility` (`self.HUDNotification`) "Hidden"))))

(event `/Game/RebelX_Core/Blueprints/Interfaces/BPI_HUD.StartReloadWarning`
  ;[1 1 1] Reloading
)

(event `ShowNotification`
  (bind _hudnotification (`self.HUDNotification`))
  ;[1 1 1] Show Notification
  (`|ExecutionSequence`
    (:`then_0`
      (set `/Game/RebelX_Core/UserInterface/W_HUDNotification.NotificationText` (`|GetArrayItem` (`self.NotificationQue`)) _hudnotification)
      (`Widget.SetVisibility` _hudnotification "Visible"))
    (:`then_1`
      (`/Game/RebelX_Core/UserInterface/W_HUDNotification.PlayAnim` (`self.HUDNotification`)))
    (:`then_2`
      (`GameplayStatics.PlaySound2D` "/Game/RebelX_Core/Audio/Weapon/SC_Pickup_Ammo.SC_Pickup_Ammo" 1.0 1.0 0.0 null null))))

(event `/Game/RebelX_Core/Blueprints/Interfaces/BPI_HUD.AddNotificaiton`
  (params (NotificationText :type Text))
  ;[1 1 1] Add notification to que
  (if (not (`KismetArrayLibrary.Array_Contains` (`self.NotificationQue`) NotificationText))
    (`KismetArrayLibrary.Array_Add` (`self.NotificationQue`) NotificationText)
    (if (not (`Widget.IsVisible` (`self.HUDNotification`)))
      (`self.ShowNotification`))))

(event `/Game/RebelX_Core/Blueprints/Interfaces/BPI_HUD.UpdateObjective`
  (params (Objective :type String) (Details :type String))
  (bind _hudcore (`self.HUDCore`))
  ;[1 1 1] Update Objective
  (set `/Game/RebelX_Core/UserInterface/HUDCore.Objective Name` (`KismetStringLibrary.Concat_StrStr` "Objective: " Objective) _hudcore)
  (set `/Game/RebelX_Core/UserInterface/HUDCore.Objective Details` (`KismetStringLibrary.Concat_StrStr` "Details: " Details) _hudcore))

(fn `UserConstructionScript`)