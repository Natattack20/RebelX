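; Player camera manager for Player_RebelX that blends the view between the first-person camera and the aim-down-sights camera.
; Player zoom events are bound on BeginPlay, and an ADS timeline, paced by the weapon's scope data, drives a lerp alpha.
; That alpha also sets scope material-collection opacity and CM_ADS modifier weight.
; BlueprintUpdateCamera lerps location and FOV by the alpha, but switches rotation instantly on the player's ADS flag.
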(event `self.ReceiveBeginPlay`
  (bind _asplayer_rebel_x (cast `/Game/RebelX_Core/Blueprints/Player_RebelX` (`Controller.K2_GetPawn` (`self.GetOwningPlayerController`)))
    (:`then`
      (bind _output_get (set `self.As Player Rebel X` _asplayer_rebel_x))
      (add `/Game/RebelX_Core/Blueprints/Player_RebelX.ZoomedIn` _output_get (`|CreateDelegate` :!event `ADS Lerp In`))
      (add `/Game/RebelX_Core/Blueprints/Player_RebelX.ZoomedOut` _output_get (`|CreateDelegate` :!event `ADS Lerp Out`))
      (bind _returnvalue (`self.AddNewCameraModifier` "/Game/RebelX_Core/Blueprints/Camera/CM_ADS.CM_ADS_C"))
      (set `self.ADS_CameraModifyer` (cast `/Game/RebelX_Core/Blueprints/Camera/CM_ADS` _returnvalue :!pure true)))
    (:`CastFailed`
      (`/Game/RebelX_Core/Blueprints/Functions/BP_DebugFunctions.DebugLog` "Failed ot cast to player." "NewEnumerator2"))))

(event `ADS Lerp In`
  (bind (_scopedata_type _scopedata_mesh _scopedata_zoommultiplyer _scopedata_adstransitionplayrate) (break `/Game/RebelX_Core/Blueprints/Structs/S_Data_Scopes` (`/Game/RebelX_Core/Blueprints/Components/BP_WeaponComponent.ScopeData` (`/Game/RebelX_Core/Blueprints/Player_RebelX.GetCurrentWeaponComponent` (`self.As Player Rebel X`)))))
  (`TimelineComponent.SetPlayRate` (`self.ADS Camera Transition`) _scopedata_adstransitionplayrate)
  (bind (_direction _lerp) (`Timeline|ADS Camera Transition` :!label _label)
    (:`Update`
      (bind _output_get (set `self.ADSLerp` _lerp))
      (`KismetMaterialLibrary.SetScalarParameterValue` "/Game/RebelX_Core/Props/Weapons/Scopes/MPC_ScopeParamaters.MPC_ScopeParamaters" "Opacity" _output_get)
      (set `/Game/RebelX_Core/Blueprints/Camera/CM_ADS.Weight` (select `/Game/RebelX_Core/Blueprints/Enums/E_ScopeType` _scopedata_type :`NewEnumerator3` _output_get :`NewEnumerator0` _output_get :`NewEnumerator1` _output_get :`NewEnumerator2` _output_get :!type "Float (double-precision)") (`self.ADS_CameraModifyer`)))))

(event `ADS Lerp Out`
  (goto _label :!via `Reverse`))

(fn `BlueprintUpdateCamera`
  (params (CameraTarget :type "Actor Object Reference"))
  (returns (NewCameraLocation :type "Vector Structure") (NewCameraRotation :type "Rotator Structure") (NewCameraFOV :type "Float (single-precision)") (ReturnValue :type Boolean))
  (locals (CameraTarget_Player :type "/Game/RebelX_Core/Blueprints/Player_RebelX Object Reference") (InterpSpeed :type "Float (single-precision)" :default 10.0))
  (bind (_cameratarget_ads_location _cameratarget_ads_rotation _cameratarget_ads_fov) (break `/Game/RebelX_Core/Blueprints/Structs/S_CameraTarget` (`self.CameraTarget_ADS`)))
  (bind (_cameratarget_current_location _cameratarget_current_rotation _cameratarget_current_fov) (break `/Game/RebelX_Core/Blueprints/Structs/S_CameraTarget` (`self.CameraTarget_Current`)))
  (bind _cameratarget_ads_location_2 (break `/Game/RebelX_Core/Blueprints/Structs/S_CameraTarget` (`self.CameraTarget_ADS`)))
  (bind _cameratarget_fp_location (break `/Game/RebelX_Core/Blueprints/Structs/S_CameraTarget` (`self.CameraTarget_FP`)))
  (bind (_cameratarget_fp_location_2 _cameratarget_fp_rotation _cameratarget_fp_fov) (break `/Game/RebelX_Core/Blueprints/Structs/S_CameraTarget` (`self.CameraTarget_FP`)))
  (bind _asplayer_rebel_x (cast `/Game/RebelX_Core/Blueprints/Player_RebelX` CameraTarget)
    (:`then`
      (bind _output_get (set `local.CameraTarget_Player` _asplayer_rebel_x))
      (bind _desiredview (`CameraComponent.GetCameraView` (`/Game/RebelX_Core/Blueprints/Player_RebelX.FirstPersonCamera` _output_get) (`GameplayStatics.GetWorldDeltaSeconds`)))
      (bind ((`Location` _location) (`Rotation` _rotation) (`FOV` _fov)) (break `MinimalViewInfo` _desiredview))
      (set `self.CameraTarget_FP` (make `/Game/RebelX_Core/Blueprints/Structs/S_CameraTarget` _location _rotation _fov))
      (bind _desiredview_2 (`CameraComponent.GetCameraView` (`/Game/RebelX_Core/Blueprints/Player_RebelX.Camera_ADS` (`local.CameraTarget_Player`)) (`GameplayStatics.GetWorldDeltaSeconds`)))
      (bind (_location_2 _rotation_2 _fov_2) (break `MinimalViewInfo` _desiredview_2))
      (set `self.CameraTarget_ADS` (make `/Game/RebelX_Core/Blueprints/Structs/S_CameraTarget` _location_2 _rotation_2 _fov_2))
      (`|ExecutionSequence`
        (:`then_0`
          (setmembers `/Game/RebelX_Core/Blueprints/Structs/S_CameraTarget` :`StructRef` (`self.CameraTarget_Current`) :`Location` (`KismetMathLibrary.VLerp` _cameratarget_fp_location _cameratarget_ads_location_2 (`self.ADSLerp`))))
        (:`then_1`
          (setmembers `/Game/RebelX_Core/Blueprints/Structs/S_CameraTarget` :`StructRef` (`self.CameraTarget_Current`) :`Rotation` (`.Rotation_7_C61CC5A043EF481EBAA5F6B783D5EC1A` (break `/Game/RebelX_Core/Blueprints/Structs/S_CameraTarget` (select `bool` (`/Game/RebelX_Core/Blueprints/Player_RebelX.bADS` (`local.CameraTarget_Player`)) :`false` (`self.CameraTarget_FP`) :`true` (`self.CameraTarget_ADS`))))))
        (:`then_2`
          (setmembers `/Game/RebelX_Core/Blueprints/Structs/S_CameraTarget` :`StructRef` (`self.CameraTarget_Current`) :`FOV` (`KismetMathLibrary.Lerp` _cameratarget_fp_fov _cameratarget_ads_fov (`self.ADSLerp`))))
        (:`then_3`
          (return _cameratarget_current_location _cameratarget_current_rotation _cameratarget_current_fov true))))
    (:`CastFailed`
      (return (0.0 0.0 0.0) (struct) 0.0 false))))

(fn `UserConstructionScript`)