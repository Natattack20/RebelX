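; Combat manager component that tracks enemies in a fight, starts and ends combat as they are added or removed, and handles chimes and music.
; A looping timer tick promotes Defensive enemies to Agressive up to a desired count, writing stances to their AI Blackboards.
; The first tick of each combat runs an EQS query for defensive positions, handed out randomly as Blackboard target locations, with spares kept for position-change requests.
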(event `StartCombat`
  (bind _enemycharachters (`self.EnemyCharachters`))
  (bind _non_combatmusic (`self.Non-CombatMusic`))
  ;[1 1 1] Start Combat
  (bind _keys (`BlueprintMapLibrary.Map_Keys` (`self.EnemyCharachters`)))
  (if (`KismetArrayLibrary.Array_IsValidIndex` _keys)
    (for _array_element _keys
      (if (not (`BlueprintMapLibrary.Map_Contains` _enemycharachters _array_element))
        (`BlueprintMapLibrary.Map_Add` _enemycharachters _array_element "NewEnumerator0")
        (`/Game/RebelX_Core/Blueprints/Functions/BP_DebugFunctions.DebugLog` (`KismetStringLibrary.Concat_StrStr` "Adding enemy to combat: " (`KismetSystemLibrary.GetDisplayName` _array_element)))))
    (bind _keys_2 (`BlueprintMapLibrary.Map_Keys` (`self.EnemyCharachters`)))
    (if (`KismetArrayLibrary.Array_IsValidIndex` _keys_2)
      (`/Game/RebelX_Core/Blueprints/Functions/BP_DebugFunctions.DebugLog` "Starting Combat")
      (set `self.bInCombat` true)
      (`self.CombatStarted`)
      (bind _returnvalue (`KismetSystemLibrary.K2_SetTimerDelegate` (delegate `CombatTick`) 5.0 true))
      (set `self.CombatActionTick` _returnvalue)
      (`self.CombatTick`)
      (`|ExecutionSequence`
        (:`then_0`
          (if (`self.bPlayCombatChimes`)
            ;[1 1 0] Need music system
            (`GameplayStatics.PlaySound2D` "/Game/RebelX_Core/Audio/FX/SC_FX_CombatStarted.SC_FX_CombatStarted" 2.0 1.0 0.0 null null)
            (`GameplayStatics.PlaySound2D` "/Game/RebelX_Core/Audio/FX/W_FX_CombatStarted.W_FX_CombatStarted" 0.5 1.0 0.0 null null)))
        (:`then_1`
          ;[1 1 0] Combat Music
          (if (`self.bPlayCombatMusic`)
            (`/Engine/EditorBlueprintResources/StandardMacros.IsValid` (`self.CombatMusic`)
              (:`Is Not Valid`
                (bind _returnvalue_2 (`GameplayStatics.SpawnSoundAttached` "/Game/RebelX_Core/Audio/FX/W_CombatMusic.W_CombatMusic" (`Actor.RootComponent` (`GameplayStatics.GetPlayerPawn` 0)) "None" (0.0 0.0 0.0) (struct) "KeepRelativeOffset" false 1.0 1.0 0.0 null null))
                (bind _output_get (set `self.CombatMusic` _returnvalue_2))
                (`AudioComponent.SetUISound` _output_get true)
                (`AudioComponent.Stop` _non_combatmusic)
                (`self.K2_DestroyComponent` _non_combatmusic)))))))
    (else
      (`/Game/RebelX_Core/Blueprints/Functions/BP_DebugFunctions.DebugLog` "Must start combat with a a valid enemy charachter" "NewEnumerator1"))))

(event `EndCombat`
  (bind _combatmusic (`self.CombatMusic`))
  ;[1 1 1] End Combat
  (`|ExecutionSequence`
    (:`then_0`
      (`BlueprintMapLibrary.Map_Clear` (`self.EnemyCharachters`))
      (set `self.bInCombat` false)
      (`self.CombatEnded`)
      (`/Game/RebelX_Core/Blueprints/Functions/BP_DebugFunctions.DebugLog` "Ending Combat")
      (`KismetSystemLibrary.K2_ClearAndInvalidateTimerHandle` (`self.CombatActionTick`))
      (`KismetSystemLibrary.Delay` 1.0)
      (`|ExecutionSequence`
        (:`then_0`
          (if (`self.bPlayCombatChimes`)
            ;[1 1 0] Need music system
            (`GameplayStatics.PlaySound2D` "/Game/RebelX_Core/Audio/FX/SC_FX_CombatEnded.SC_FX_CombatEnded" 2.0 1.0 0.0 null null)))
        (:`then_1`
          (`/Engine/EditorBlueprintResources/StandardMacros.IsValid` _combatmusic
            (:`Is Valid`
              (`AudioComponent.Stop` _combatmusic)
              (`self.K2_DestroyComponent` _combatmusic)
              (bind _returnvalue (`GameplayStatics.SpawnSoundAttached` "/Game/AMD/Nathan/Audio/Prison_Ambience.Prison_Ambience" (`Actor.RootComponent` (`GameplayStatics.GetPlayerPawn` 0)) "None" (0.0 0.0 0.0) (struct) "KeepRelativeOffset" false 1.0 1.0 0.0 null null))
              (set `self.Non-CombatMusic` _returnvalue))))))
    (:`then_1`
      (goto _label :!via `Reset`))))

(event `ForceCombatTick`
  ;[1 1 1] Force update combat tick
  (bind _returnvalue (`KismetSystemLibrary.K2_SetTimerDelegate` (delegate `CombatTick`) 5.0 true))
  (set `self.CombatActionTick` _returnvalue)
  (`self.CombatTick`))

(event `CombatTick`
  (bind _enemycharachters (`self.EnemyCharachters`))
  (bind _totalagressive (`self.TotalAgressive`))
  ;[1 1 1] Combat Tick
  (`/Game/RebelX_Core/Blueprints/Functions/BP_DebugFunctions.DebugLog` "Combat Tick")
  (`|ExecutionSequence`
    (:`then_0`
      (set `self.TotalAgressive` 0)
      (bind _keys (`BlueprintMapLibrary.Map_Keys` _enemycharachters))
      (for _array_element _keys
        (if (`|EnumEquality` (`BlueprintMapLibrary.Map_Find` _enemycharachters _array_element) "NewEnumerator2")
          (if (>= _totalagressive (`self.DesiredAgressive`))
            (`self.SetCharachterStance` _array_element "NewEnumerator2")
            (else
              (`/Engine/EditorBlueprintResources/StandardMacros.IncrementInt` _totalagressive
                (:`  `
                  (`self.SetCharachterStance` _array_element "NewEnumerator1"))))))))
    (:`then_1`
      (`/Engine/EditorBlueprintResources/StandardMacros.DoOnce` false :!label _label
        (:`Completed`
          (bind _keys_2 (`BlueprintMapLibrary.Map_Keys` (`self.EnemyCharachters`)))
          (bind _returnvalue (`EnvQueryManager.RunEQSQuery` "/Game/RebelX_Core/Blueprints/AI/EQS/FindDefensivePositions.FindDefensivePositions" (`|GetArrayItem` _keys_2) "AllMatching"))
          (bind _output_get (set `self.EQS` _returnvalue))
          (add `EnvQueryInstanceBlueprintWrapper.OnQueryFinishedEvent` _output_get (delegate `EQSFinished`)))))))

(event `self.ReceiveBeginPlay`
  ;[1 1 1] Combat Tick
)

(event `EQSFinished`
  (params (QueryInstance :type "EnvQueryInstanceBlueprintWrapper Object Reference") (QueryStatus :type "EEnvQueryStatus Enum" :default "Processing"))
  ;[1 1 1] Combat Tick
  (bind (_resultlocations _returnvalue) (`EnvQueryInstanceBlueprintWrapper.GetQueryResultsAsLocations` QueryInstance))
  (if _returnvalue
    (bind _output_get (set `self.AvaliblePositions` _resultlocations))
    (`self.Find Defensive Position` _output_get)
    (else
      (`/Game/RebelX_Core/Blueprints/Functions/BP_DebugFunctions.DebugLog` "EQS Failed" "NewEnumerator1"))))

(fn `AddEnemyToCombat`
  (params (Charachter :type "/Game/RebelX_Core/Blueprints/AI/BP_Master_Enemy Object Reference"))
  (`/Engine/EditorBlueprintResources/StandardMacros.IsValid` Charachter
    (:`Is Valid`
      (`|ExecutionSequence`
        (:`then_0`
          (if (not (`BlueprintMapLibrary.Map_Contains` (`self.EnemyCharachters`) Charachter))
            (`self.SetCharachterStance` Charachter "NewEnumerator2")
            (`self.EnemyAdded`)
            (else
              (`/Game/RebelX_Core/Blueprints/Functions/BP_DebugFunctions.DebugLog` "Charachter already in combat" "NewEnumerator1"))))
        (:`then_1`
          (bind _keys (`BlueprintMapLibrary.Map_Keys` (`self.EnemyCharachters`)))
          (if (`KismetArrayLibrary.Array_IsValidIndex` _keys)
            (if (not (`self.bInCombat`))
              (`self.StartCombat`))))))
    (:`Is Not Valid`
      (`/Game/RebelX_Core/Blueprints/Functions/BP_DebugFunctions.DebugLog` "Invalid Charachter. Cannot add to combat" "NewEnumerator1"))))

(fn `Find Defensive Position`
  (params (Postions :type "Array of Vector Structure"))
  (locals (TempPositions :type "Array of Vector Structure") (TempCurrentItem :type "Vector Structure"))
  (bind _temppositions (`local.TempPositions`))
  (set `local.TempPositions` Postions)
  (`|ExecutionSequence`
    (:`then_0`
      (bind _keys (`BlueprintMapLibrary.Map_Keys` (`self.EnemyCharachters`)))
      (for _array_element _keys
        (bind _output_get (set `local.TempCurrentItem` (`|GetArrayItem` _temppositions (`KismetMathLibrary.RandomIntegerInRange` 0 (`KismetArrayLibrary.Array_Length` _temppositions)))))
        (if (not (`BlueprintMapLibrary.Map_Contains` (`self.EnemyPositions`) _array_element))
          (`self.SetCharachterTargetPosition` _array_element _output_get)
          (`KismetArrayLibrary.Array_RemoveItem` (`local.TempPositions`) _output_get))))
    (:`then_1`
      (set `self.AvaliblePositions` (`local.TempPositions`))
      (return))))

(fn `RemoveEnemyFromCombat`
  (params (Charachter :type "/Game/RebelX_Core/Blueprints/AI/BP_Master_Enemy Object Reference"))
  (bind _enemycharachters (`self.EnemyCharachters`))
  (if (`BlueprintMapLibrary.Map_Contains` (`self.EnemyCharachters`) Charachter)
    (switch `/Game/RebelX_Core/Blueprints/Enums/E_EnemyStances` (`BlueprintMapLibrary.Map_Find` _enemycharachters Charachter)
      (:`NewEnumerator0`
        _)
      (:`NewEnumerator1`
        (`/Engine/EditorBlueprintResources/StandardMacros.DecrementInt` (`self.TotalAgressive`)
          (:`  `
            _)))
      (:`NewEnumerator2`
        _)
      (:`NewEnumerator3`
        _))
    (`BlueprintMapLibrary.Map_Remove` _enemycharachters Charachter)
    (`self.EnemyRemoved`)
    (bind _keys (`BlueprintMapLibrary.Map_Keys` _enemycharachters))
    (if (`KismetArrayLibrary.Array_IsValidIndex` _keys)
      (`self.ForceCombatTick`)
      (else
        (`self.EndCombat`)))
    (else
      (`/Game/RebelX_Core/Blueprints/Functions/BP_DebugFunctions.DebugLog` "Cannot remove charachter from combat as they were not in combat" "NewEnumerator1"))))

(fn `RequestPositionChange`
  (params (Enemy :type "/Game/RebelX_Core/Blueprints/AI/BP_Master_Enemy Object Reference"))
  (locals (Temp_Position :type "Vector Structure"))
  (bind _avaliblepositions (`self.AvaliblePositions`))
  (if (`.ReturnValue` (`BlueprintMapLibrary.Map_Find` (`self.EnemyPositions`) Enemy))
    (bind _output_get (set `local.Temp_Position` (`|GetArrayItem` _avaliblepositions (`KismetMathLibrary.RandomIntegerInRange` 0 (`KismetArrayLibrary.Array_Length` _avaliblepositions)))))
    (`KismetArrayLibrary.Array_RemoveItem` _avaliblepositions _output_get)
    (`self.SetCharachterTargetPosition` Enemy _output_get)
    (`KismetSystemLibrary.DrawDebugSphere` _output_get 100.0 12 (struct :`G` 1.0 :`A` 1.0) 5.0 3.0)
    (`KismetSystemLibrary.PrintString` (`KismetStringLibrary.Concat_StrStr` "Remaining Positions" (`KismetStringLibrary.Conv_IntToString` (`KismetArrayLibrary.Array_Length` (`self.AvaliblePositions`)))))
    (else
      (`/Game/RebelX_Core/Blueprints/Functions/BP_DebugFunctions.DebugLog` "Enemy position not known" "NewEnumerator1"))))

(fn `SendToAttack`
  (params (Charachter :type "Character Object Reference"))
  (`BlackboardComponent.SetValueAsEnum` (`AIBlueprintHelperLibrary.GetBlackboard` (`AIBlueprintHelperLibrary.GetAIController` Charachter)) "Stance" (enumliteral `/Game/RebelX_Core/Blueprints/Enums/E_EnemyStances` "NewEnumerator1")))

(fn `SetCharachterStance`
  (params (ControlledEnemy :type "/Game/RebelX_Core/Blueprints/AI/BP_Master_Enemy Object Reference") (Stance :type "/Game/RebelX_Core/Blueprints/Enums/E_EnemyStances Enum" :default "NewEnumerator0"))
  (`BlueprintMapLibrary.Map_Add` (`self.EnemyCharachters`) ControlledEnemy Stance)
  (`BlackboardComponent.SetValueAsEnum` (`AIBlueprintHelperLibrary.GetBlackboard` (`AIBlueprintHelperLibrary.GetAIController` ControlledEnemy)) "Stance" Stance))

(fn `SetCharachterTargetPosition`
  (params (Charachter :type "/Game/RebelX_Core/Blueprints/AI/BP_Master_Enemy Object Reference") (NewPosition :type "Vector Structure"))
  (`BlueprintMapLibrary.Map_Add` (`self.EnemyPositions`) Charachter NewPosition)
  (`BlackboardComponent.SetValueAsVector` (`AIBlueprintHelperLibrary.GetBlackboard` (`AIBlueprintHelperLibrary.GetAIController` Charachter)) "TargetLocation" NewPosition))

(fn `UpdateCombatParamaters`
  (params (DesiredAgressive :type Integer) (bPlayCombatMusic :type Boolean) (bPlayCombatChimes :type Boolean))
  (set `self.DesiredAgressive` DesiredAgressive)
  (set `self.bPlayCombatMusic` bPlayCombatMusic)
  (set `self.bPlayCombatChimes` bPlayCombatChimes))