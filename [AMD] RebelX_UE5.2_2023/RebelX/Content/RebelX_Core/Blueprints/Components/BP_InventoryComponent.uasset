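; Inventory component that tracks ammo per type and a count of distraction throwables.
; On BeginPlay, when the game instance's FirstTime is false, ResetAmmo scales each max by a multiplier and adds starting ammo based on that max.
; Add and consume functions write clamped struct copies back to the Ammo map, report actual amounts and dispatch full or depleted events, with UnlimitedAmmo bypassing consumption.
; Throwables use only the Distraction counter; Grenades logic is disconnected.
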(event `self.ReceiveBeginPlay`
  ;[1 1 1] Begin Play
  (if (not (`/Game/AMD/Instance.FirstTime?` (cast `/Game/AMD/Instance` (`GameplayStatics.GetGameInstance`) :!pure true)))
    (`self.ResetAmmo`)
    (`KismetSystemLibrary.PrintString` "Hello")))

(event `ResetAmmo`
  ;[1 1 1] Reset Ammo
  (bind _keys (`BlueprintMapLibrary.Map_Keys` (`self.Ammo`)))
  (for _array_element _keys
    (bind (_avalible _maxallowed) (`self.GetAmmoOfType` _array_element))
    (`BlueprintMapLibrary.Map_Add` (`self.Ammo`) _array_element (make `/Game/RebelX_Core/Blueprints/Structs/S_Inv_Ammo` _avalible (* _maxallowed (`self.MaxAmmoMultiplier `)))) ; Update max ammo from modifyer
    (`self.AddAmmo` _array_element (* (`self.StartingAmmoMultiplier `) (/ _maxallowed 4)))))

(fn `AddAmmo`
  (params (AmmoType :type "/Game/RebelX_Core/Blueprints/Enums/E_WeaponTypes Enum" :default "NewEnumerator0") (Quantity :type Integer))
  (returns (FullAmmoType :type Boolean) (TotalAdded :type Integer))
  (locals (Temp_TotalAdded :type Integer) (Temp_PreviousAvalible :type Integer))
  (bind (_value _returnvalue) (`BlueprintMapLibrary.Map_Find` (`self.Ammo`) (`local.AmmoType`)))
  (bind (_avalible _maxallowed) (break `/Game/RebelX_Core/Blueprints/Structs/S_Inv_Ammo` _value))
  (bind (_avalible_2 _maxallowed_2) (break `/Game/RebelX_Core/Blueprints/Structs/S_Inv_Ammo` (`BlueprintMapLibrary.Map_Find` (`self.Ammo`) (`local.AmmoType`))))
  (bind _returnvalue_2 (== _avalible_2 _maxallowed_2))
  (`|ExecutionSequence`
    (:`then_0`
      ;[1 1 1] Log Desired
      (`/Game/RebelX_Core/Blueprints/Functions/BP_DebugFunctions.DebugLog` (`KismetStringLibrary.Concat_StrStr` "Adding " (`|GetEnumeratorNameAsString` (`local.AmmoType`)) " Ammo" "(" (`KismetStringLibrary.Conv_IntToString` (`local.Quantity`)) ")")))
    (:`then_1`
      ;[1 1 1] Add ammo to map
      (if _returnvalue
        (set `local.Temp_PreviousAvalible` _avalible) ; For calculating total actually added
        (bind _structout (setmembers `/Game/RebelX_Core/Blueprints/Structs/S_Inv_Ammo` :`StructRef` _value :`Avalible` (`KismetMathLibrary.Clamp` (+ _avalible (`local.Quantity`)) 0 _maxallowed)))
        (`BlueprintMapLibrary.Map_Add` (`self.Ammo`) (`local.AmmoType`) _structout) ; Update Map with copy
        (else
          ;[1 1 1] Add new ammo type
          (`/Game/RebelX_Core/Blueprints/Functions/BP_DebugFunctions.DebugLog` "Adding new ammo type")
          (`BlueprintMapLibrary.Map_Add` (`self.Ammo`) (`local.AmmoType`) (make `/Game/RebelX_Core/Blueprints/Structs/S_Inv_Ammo` (`local.Quantity`) 100)) ; Update Map with copy
        )))
    (:`then_2`
      ;[1 1 1] Log new total ammo
      (`/Game/RebelX_Core/Blueprints/Functions/BP_DebugFunctions.DebugLog` (`KismetStringLibrary.Concat_StrStr` "New " (`|GetEnumeratorNameAsString` (`local.AmmoType`)) " Ammo" "(" (`KismetStringLibrary.Conv_IntToString` (`.Avalible_13_A2BCF8A642CF79B49FC5018AD8EFA8E3` (break `/Game/RebelX_Core/Blueprints/Structs/S_Inv_Ammo` (`BlueprintMapLibrary.Map_Find` (`self.Ammo`) (`local.AmmoType`))))) ")")))
    (:`then_3`
      ;[1 1 1] Dispatch if full
      (if _returnvalue_2
        (`self.AmmoFull` (`local.AmmoType`))))
    (:`then_4`
      ;[1 1 1] Output results
      (return _returnvalue_2 (- _avalible_2 (`local.Temp_PreviousAvalible`))))))

(fn `AddThrowable`
  (params (Count :type Integer))
  (set `self.Distraction` (+ Count (`self.Distraction`))))

(fn `ConsumeAmmo`
  (params (AmmoType :type "/Game/RebelX_Core/Blueprints/Enums/E_WeaponTypes Enum" :default "NewEnumerator0") (AmountToConsume :type Integer))
  (returns (AmountConsumed :type Integer) (MissingAmmo :type Boolean) (TotalMissing :type Integer))
  (locals (Temp_TotalMissing :type Integer :default 0))
  (bind _temp_totalmissing (`local.Temp_TotalMissing`))
  (bind _ammotype (`local.AmmoType`))
  (bind (_avalible _maxallowed) (break `/Game/RebelX_Core/Blueprints/Structs/S_Inv_Ammo` (`BlueprintMapLibrary.Map_Find` (`self.Ammo`) (`local.AmmoType`))))
  (bind _returnvalue (- (`.Avalible_13_A2BCF8A642CF79B49FC5018AD8EFA8E3` (break `/Game/RebelX_Core/Blueprints/Structs/S_Inv_Ammo` (`BlueprintMapLibrary.Map_Find` (`self.Ammo`) (`local.AmmoType`)))) (`local.AmountToConsume`)))
  (if (`self.UnlimitedAmmo`)
    (return AmountToConsume false 0)
    (else
      (`|ExecutionSequence`
        (:`then_0`
          ;[1 1 1] Log Desired
          (`/Game/RebelX_Core/Blueprints/Functions/BP_DebugFunctions.DebugLog` (`KismetStringLibrary.Concat_StrStr` "Consuming " (`|GetEnumeratorNameAsString` (`local.AmmoType`)) " Ammo" "(" (`KismetStringLibrary.Conv_IntToString` (`local.AmountToConsume`)) ")")))
        (:`then_1`
          ;[1 1 1] Check for missing ammo
          (if (< _returnvalue 0)
            (set `local.Temp_TotalMissing` (`KismetMathLibrary.Abs_Int` _returnvalue))))
        (:`then_2`
          ;[1 1 1] Consume Ammo
          (bind _structout (setmembers `/Game/RebelX_Core/Blueprints/Structs/S_Inv_Ammo` :`StructRef` (`BlueprintMapLibrary.Map_Find` (`self.Ammo`) (`local.AmmoType`)) :`Avalible` (`KismetMathLibrary.Clamp` (- _avalible (`local.AmountToConsume`)) 0 _maxallowed)))
          (`BlueprintMapLibrary.Map_Add` (`self.Ammo`) (`local.AmmoType`) _structout) ; Update map with copy
        )
        (:`then_3`
          ;[1 1 1] Log resluts
          (`/Game/RebelX_Core/Blueprints/Functions/BP_DebugFunctions.DebugLog` (`KismetStringLibrary.Concat_StrStr` "Comsumed  " (`|GetEnumeratorNameAsString` (`local.AmmoType`)) " Ammo" "(" (`KismetStringLibrary.Conv_IntToString` (- (`local.AmountToConsume`) (`local.Temp_TotalMissing`))) ")")))
        (:`then_4`
          ;[1 1 1] Dispatch if depleted
          (if (== (`.Avalible_13_A2BCF8A642CF79B49FC5018AD8EFA8E3` (break `/Game/RebelX_Core/Blueprints/Structs/S_Inv_Ammo` (`BlueprintMapLibrary.Map_Find` (`self.Ammo`) _ammotype))) 0)
            (`self.AmmoDepleted` _ammotype)))
        (:`then_5`
          ;[1 1 1] Output Results
          (return (- (`local.AmountToConsume`) _temp_totalmissing) (> _temp_totalmissing 0) (`local.Temp_TotalMissing`)))))))

(fn `ConsumeThrowable`
  (returns (ReturnValu :type Boolean) (Type :type String))
  (bind _distraction (`self.Distraction`))
  (if (not (< (- _distraction 1) 0))
    (`/Engine/EditorBlueprintResources/StandardMacros.DecrementInt` _distraction
      (:`  `
        (return true "Distraction")))
    (else
      (return false "Distraction"))))

(fn `GetAmmoOfType`
  (params (AmmoType :type "/Game/RebelX_Core/Blueprints/Enums/E_WeaponTypes Enum" :default "NewEnumerator0"))
  (returns (Avalible :type Integer) (MaxAllowed :type Integer) (ReturnValue :type Boolean))
  (bind (_value _returnvalue) (`BlueprintMapLibrary.Map_Find` (`self.Ammo`) AmmoType))
  (return (break `/Game/RebelX_Core/Blueprints/Structs/S_Inv_Ammo` _value) (`.MaxAllowed_14_BDF8B6B8447B3EA60381209E4F2D0F33` (break `/Game/RebelX_Core/Blueprints/Structs/S_Inv_Ammo` _value)) _returnvalue))