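; BP_Master_Enemy is the base enemy Blueprint, handling entry into and exit from combat.
; Damage from a player updates the AI controller's target, alerts this enemy and nearby ones via sphere overlap, and feeds the health component.
; Alerted enemies register once with the game mode's combat manager component, and deregister when health depletes, firing Alerted and Eliminated calls respectively.
; GetWeapon and StartFire are empty stubs.
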(event `self.ReceiveAnyDamage`
  (params (Damage :type "Float (single-precision)") (DamageType :type "DamageType Object Reference") (InstigatedBy :type "Controller Object Reference") (DamageCauser :type "Actor Object Reference"))
  ;[1 1 1] Recive Damage
  (`|ExecutionSequence`
    (:`then_0`
      (if (`self.IsAIControllerValid`)
        (bind _asplayer_rebel_x (cast `/Game/RebelX_Core/Blueprints/Player_RebelX` (`Actor.Instigator` DamageCauser)))
        (`/Game/RebelX_Core/Blueprints/AI/AIController_Enemy.UpdateTarget` (cast `/Game/RebelX_Core/Blueprints/AI/AIController_Enemy` (`AIBlueprintHelperLibrary.GetAIController` self) :!pure true) _asplayer_rebel_x)
        (`self.AlertToCombat` _asplayer_rebel_x)
        (`self.AlertNearby` _asplayer_rebel_x)))
    (:`then_1`
      (`/Game/RebelX_Core/Blueprints/Components/BP_HealthComponent.TakeDamage` (`self.BP_HealthComponent`) Damage DamageType))))

(event `AlertNearby`
  (params (NewTarget :type "Actor Object Reference"))
  ;[1 1 1] Alert others to combat
  (bind _outactors (`KismetSystemLibrary.SphereOverlapActors` (`self.K2_GetActorLocation`) 2500.0 (`|MakeArray` "ObjectTypeQuery3" :!type "EObjectTypeQuery Enum") "BP_Master_Enemy_C" (`|MakeArray` self :!type "Actor Object Reference")))
  (for _array_element _outactors
    (`self.AlertToCombat` (cast `/Game/RebelX_Core/Blueprints/AI/BP_Master_Enemy` _array_element :!pure true) NewTarget)))

(event `AlertToCombat`
  (params (NewTarget :type "Actor Object Reference"))
  ;[1 1 1] Alert to Combat
  (if (not (`self.InCombat`))
    (bind _asaicontroller_enemy (cast `/Game/RebelX_Core/Blueprints/AI/AIController_Enemy` (`AIBlueprintHelperLibrary.GetAIController` self))
      (:`then`
        (`/Game/RebelX_Core/Blueprints/AI/AIController_Enemy.UpdateTarget` _asaicontroller_enemy NewTarget))
      (:`CastFailed`
        _))
    (`/Game/RebelX_Core/Blueprints/Components/BP_CombatManager.AddEnemyToCombat` (`self.GetCombatManager`) self)
    (set `self.InCombat` true)
    (`self.Alerted`)))

(event `self.BP_HealthComponent.HealthDepleted`
  ;[1 1 1] Remove From Combat
  (`/Engine/EditorBlueprintResources/StandardMacros.DoOnce` false
    (:`Completed`
      (`self.Eliminated` self)
      (`/Game/RebelX_Core/Blueprints/Components/BP_CombatManager.RemoveEnemyFromCombat` (`self.GetCombatManager`) self))))

(fn `GetCombatManager`
  (returns (CombatManager :type "/Game/RebelX_Core/Blueprints/Components/BP_CombatManager Object Reference"))
  (return (`self.GetComponentByClass` (`GameplayStatics.GetGameMode`) "/Game/RebelX_Core/Blueprints/Components/BP_CombatManager.BP_CombatManager_C")))

(fn `GetWeapon`
  (returns (Weapon :type "/Game/RebelX_Core/Blueprints/Components/BP_WeaponComponent Object Reference"))
  (return null))

(fn `IsAIControllerValid`
  (returns (ReturnValue :type Boolean))
  (return (`KismetSystemLibrary.IsValid` (`AIBlueprintHelperLibrary.GetAIController` self))))

(fn `StartFire`
  (returns (WeaponComp :type "/Game/RebelX_Core/Blueprints/Components/BP_WeaponComponent Object Reference"))
  (return null))

(fn `UserConstructionScript`)