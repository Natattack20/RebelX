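; BP_Target is a damage test target that shows the damage it takes as floating text.
; Each point damage hit adds to a running total, reveals the text render with that total and starts a one-second timer.
; When the timer fires, the text hides and the total resets to zero, so hits in quick succession accumulate into one readout.
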(event `self.ReceiveTick`
  (params (DeltaSeconds :type "Float (single-precision)")))

(event `self.ReceiveBeginPlay`)

(event `Countdown`
  (`SceneComponent.SetHiddenInGame` (`self.TextRender`) true false)
  (set `self.DmgScore` 0.0))

(event `self.ReceivePointDamage`
  (params (Damage :type "Float (single-precision)") (DamageType :type "DamageType Object Reference") (HitLocation :type "Vector Structure") (HitNormal :type "Vector Structure") (HitComponent :type "PrimitiveComponent Object Reference") (BoneName :type Name) (ShotFromDirection :type "Vector Structure") (InstigatedBy :type "Controller Object Reference") (DamageCauser :type "Actor Object Reference") (HitInfo :type "HitResult Structure (by ref)"))
  (bind _output_get (set `self.DmgScore` (+ (`self.DmgScore`) Damage)))
  (`SceneComponent.SetHiddenInGame` (`self.TextRender`) false false)
  (`TextRenderComponent.K2_SetText` (`self.TextRender`) (`|FormatText` "{Damage} dmg" _output_get))
  (bind _returnvalue (`KismetSystemLibrary.K2_SetTimerDelegate` (delegate `Countdown`) 1.0))
  (set `self.DmgTimer` _returnvalue))

(fn `UserConstructionScript`)