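; BP_Damage_Volume is a box volume that deals periodic damage to Characters inside it.
; The first Character to begin overlapping the box starts a looping timer, with no damage until its first interval elapses.
; Each timer tick applies the per-tick damage to every overlapping Character, with the volume as damage causer.
; When an end overlap leaves no Characters inside, the timer is cleared, so the volume avoids Tick entirely.
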(event `self.Box.OnComponentBeginOverlap`
  (params (OverlappedComponent :type "PrimitiveComponent Object Reference") (OtherActor :type "Actor Object Reference") (OtherComp :type "PrimitiveComponent Object Reference") (OtherBodyIndex :type Integer) (bFromSweep :type Boolean) (SweepResult :type "HitResult Structure (by ref)"))
  (if (not (`KismetSystemLibrary.K2_IsValidTimerHandle` (`self.DamageTickTimer`)))
    (cast `Character` OtherActor)
    (bind _returnvalue (`KismetSystemLibrary.K2_SetTimerDelegate` (delegate `DamageOverlapping`) (`self.DamageTickDuration`) true))
    (set `self.DamageTickTimer` _returnvalue)))

(event `DamageOverlapping`
  (for _array_element (`self.GetOverlappingActors` "/Script/Engine.Character")
    (`GameplayStatics.ApplyDamage` _array_element (`self.DamagePerTick`) null self)))

(event `self.Box.OnComponentEndOverlap`
  (params (OverlappedComponent :type "PrimitiveComponent Object Reference") (OtherActor :type "Actor Object Reference") (OtherComp :type "PrimitiveComponent Object Reference") (OtherBodyIndex :type Integer))
  (if (not (`KismetArrayLibrary.Array_IsValidIndex` (`self.GetOverlappingActors` "/Script/Engine.Character")))
    (`KismetSystemLibrary.K2_ClearAndInvalidateTimerHandle` (`self.DamageTickTimer`))))

(fn `UserConstructionScript`)