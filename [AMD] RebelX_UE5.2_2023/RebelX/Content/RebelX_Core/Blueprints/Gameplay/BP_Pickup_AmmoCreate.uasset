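; BP_Pickup_AmmoCreate is an ammo pickup interactable that is flagged as non-consumable.
; GetInteractionType supplies its interaction type and prompt, while GetAmmoInfo returns a map granting the same fixed amount for eight ammo types.
; AttemptConsumeInteractable is empty, so the actor only reports data and does nothing when consumed.
; The construction script holds disconnected dynamic-material code for bullet and shell decals, which never runs.
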(event `/Game/RebelX_Core/Blueprints/Interfaces/BPI_Interactables.AttemptConsumeInteractable`)

(fn `GetAmmoInfo`
  (returns (`Return Value` :type Boolean) (Ammo :type "Map of /Game/RebelX_Core/Blueprints/Enums/E_WeaponTypes Enum to Integer"))
  (return true (`|MakeMap` "NewEnumerator5" 99 "NewEnumerator4" 99 "NewEnumerator2" 99 "NewEnumerator1" 99 "NewEnumerator6" 99 "NewEnumerator3" 99 "NewEnumerator7" 99 "NewEnumerator0" 99 :!type "/Game/RebelX_Core/Blueprints/Enums/E_WeaponTypes Enum")))

(fn `GetInteractionType`
  (returns (`Return Value` :type Boolean) (InteractionType :type "/Game/RebelX_Core/Blueprints/Enums/E_InteractionTyoes Enum") (Consumeable :type Boolean) (InteractionMessage :type Text) (IconBrush :type "SlateBrush Structure"))
  (return true "NewEnumerator1" false "..."))

(fn `UserConstructionScript`)