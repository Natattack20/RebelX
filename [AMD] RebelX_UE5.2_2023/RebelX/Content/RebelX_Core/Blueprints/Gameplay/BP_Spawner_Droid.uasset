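; Droid spawner that replaces hand-placed enemies with timed waves of teleport-in spawns.
; The construction script bakes each mapped enemy's class, transform, weapon and waypoints, marking it with a debug arrow.
; BeginPlay caches that data, destroys the placed actors and optionally auto-activates.
; A delayed recursive loop spawns current-wave entries with effects; emptying the active enemy list starts the next wave until all are defeated.
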(event `self.ReceiveBeginPlay`
  (bind _enemyspawns (`self.EnemySpawns`))
  (`|ExecutionSequence`
    (:`then_0`
      (`KismetArrayLibrary.Array_Clear` (`self.SpawnData`))
      (bind _keys (`BlueprintMapLibrary.Map_Keys` _enemyspawns))
      (for _array_element _keys
        (`KismetArrayLibrary.Array_Add` (`self.SpawnData`) (`BlueprintMapLibrary.Map_Find` _enemyspawns _array_element))
        (`self.K2_DestroyActor` _array_element)))
    (:`then_1`
      ;[1 1 1] Auto Activate
      (if (`self.AutoActivate`)
        (`self.ActivateSpawner`)))))

(event `ActivateSpawner`
  ;[1 1 1] Activate Spawner
  (`self.StartWave`))

(event `StartWave`
  ;[1 1 1] Start Wave
  (bind _result (`/Engine/EditorBlueprintResources/StandardMacros.IncrementInt` (`self.CurrentWave`))
    (:`  `
      (if (> _result (`self.Waves`))
        (`self.AllWavesDefeated`)
        (else
          (`self.Spawn`))))))

(event `Spawn`
  (bind _index (`self.INdex`))
  (bind _currentspawntransform (`self.CurrentSpawnTransform`))
  (bind _location (.location _currentspawntransform))
  (bind (_class _transform _startingweapon _wave _waypoints) (break `/Game/RebelX_Core/Blueprints/Structs/S_EnemySpawnInfo` (`|GetArrayItem` (`self.SpawnData`) (`self.INdex`))))
  ;[1 1 1] Spawn Loop
  (`|ExecutionSequence`
    (:`then_0`
      (set `self.CurrentSpawnTransform` _transform)
      (if (== _wave (`self.CurrentWave`))
        (`GameplayStatics.PlaySoundAtLocation` "/Game/RebelX_Core/Audio/Droid/W_Droid_Teleport.W_Droid_Teleport" _location (struct) 1.0 1.0 0.0 null null null null)
        (`NiagaraFunctionLibrary.SpawnSystemAtLocation` "/Game/RebelX_Core/VFX/Explosions/Systems/NS_Distortion.NS_Distortion" _location (struct) (0.1 0.1 0.1))
        (bind _returnvalue (`|SpawnActorFromClass` _class _currentspawntransform "AdjustIfPossibleButAlwaysSpawn" "SelectDefaultAtRuntime" null _startingweapon null))
        (bind _asai_soldier_child (cast `/Game/RebelX_Core/Blueprints/AI/_Soldier/AI_Soldier_Child` _returnvalue :!pure true))
        (`/Engine/EditorBlueprintResources/StandardMacros.IsValid` _asai_soldier_child
          (:`Is Valid`
            (set `/Game/RebelX_Core/Blueprints/AI/_Soldier/AI_Soldier.Waypoints` _waypoints _asai_soldier_child))
          (:`Is Not Valid`
            _))
        (`KismetArrayLibrary.Array_Add` (`self.ActiveEnemies`) _returnvalue)
        (add `self.OnDestroyed` _returnvalue (delegate `AIDefeated`))))
    (:`then_1`
      (`KismetSystemLibrary.Delay` (+ (`self.DelayBetweenSpawns`) (* (`self.DelayVariation`) (`KismetMathLibrary.Conv_BoolToDouble` (`KismetMathLibrary.RandomBool`)))))
      (`/Engine/EditorBlueprintResources/StandardMacros.IncrementInt` _index
        (:`  `
          (if (> _index (`KismetArrayLibrary.Array_LastIndex` (`self.SpawnData`)))
            (set `self.INdex` 0)
            (else
              (`self.Spawn`))))))))

(event `AIDefeated` :!signature `self.OnDestroyed`
  (params (DestroyedActor :type "Actor Object Reference"))
  (bind _activeenemies (`self.ActiveEnemies`))
  ;[1 1 1] Enemey Destroyed
  (bind _asbp_master_enemy (cast `/Game/RebelX_Core/Blueprints/AI/BP_Master_Enemy` DestroyedActor))
  (`KismetArrayLibrary.Array_RemoveItem` _activeenemies _asbp_master_enemy)
  (if (== (`KismetArrayLibrary.Array_LastIndex` _activeenemies) -1)
    (`self.WaveDefeated`)
    (`self.StartWave`)))

(fn `UserConstructionScript`
  (bind _enemyspawns (`self.EnemySpawns`))
  (`KismetArrayLibrary.Array_Clear` (`self.SpawnData`))
  (bind _keys (`BlueprintMapLibrary.Map_Keys` _enemyspawns))
  (for _array_element _keys
    (bind (_value _returnvalue) (`BlueprintMapLibrary.Map_Find` _enemyspawns _array_element))
    (if _returnvalue
      (`BlueprintMapLibrary.Map_Add` _enemyspawns _array_element (make `/Game/RebelX_Core/Blueprints/Structs/S_EnemySpawnInfo` (`GameplayStatics.GetObjectClass` _array_element) (`self.GetTransform` _array_element) (`/Game/RebelX_Core/Blueprints/AI/BP_Master_Enemy.StartingWeapon` _array_element) (`.Wave_6_E6EDC9534C5ECEA1EB04FDBBC3CA7388` (break `/Game/RebelX_Core/Blueprints/Structs/S_EnemySpawnInfo` _value)) (`/Game/RebelX_Core/Blueprints/AI/_Soldier/AI_Soldier.Waypoints` (cast `/Game/RebelX_Core/Blueprints/AI/_Soldier/AI_Soldier_Child` _array_element :!pure true))))
      (bind _returnvalue_2 (`self.K2_GetActorLocation` _array_element))
      (`KismetSystemLibrary.DrawDebugArrow` (+ _returnvalue_2 (0.0 0.0 250.0)) _returnvalue_2 0.0 (struct :`B` 1.0 :`A` 1.0) 5.0 50.0))))