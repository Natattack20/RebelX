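; Weapon pickup actor that reports itself as a consumable interaction with the weapon's name and icon, and hands out its WeaponStats.
; Init runs on construction and BeginPlay, loading stats by row name with type-based row previews, or using existing stats for spawned weapons.
; It sets meshes, lists compatible scopes and aligns the scope via its S_Offset socket.
; BeginPlay sets the player's HasGun immediately, before any pickup.
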(event `self.ReceiveBeginPlay`
  (bind _asplayer_rebel_x (cast `/Game/RebelX_Core/Blueprints/Player_RebelX` (`GameplayStatics.GetPlayerCharacter` 0)))
  (bind _output_get (set `self.As Player Rebel X` _asplayer_rebel_x))
  (set `/Game/RebelX_Core/Blueprints/Player_RebelX.HasGun` true _output_get)
  (`self.Init`))

(fn `GetInteractionType`
  (returns (`Return Value` :type Boolean) (InteractionType :type "/Game/RebelX_Core/Blueprints/Enums/E_InteractionTyoes Enum") (Consumeable :type Boolean) (InteractionMessage :type Text) (IconBrush :type "SlateBrush Structure"))
  (bind (_displayname _icon) (break `/Game/RebelX_Core/Blueprints/Structs/S_Weapon_UI` (`.UI_105_18C09244462A2AA81C3EF7A5585B0A40` (break `/Game/RebelX_Core/Blueprints/Structs/S_Data_Weapon` (`self.WeaponStats`)))))
  (return true "NewEnumerator5" true _displayname _icon))

(fn `GetWeaponInfo`
  (returns (`Return Value` :type Boolean) (`Weapon Data` :type "/Game/RebelX_Core/Blueprints/Structs/S_Data_Weapon Structure"))
  (return true (`self.WeaponStats`)))

(fn `UserConstructionScript`
  (`self.Init`))