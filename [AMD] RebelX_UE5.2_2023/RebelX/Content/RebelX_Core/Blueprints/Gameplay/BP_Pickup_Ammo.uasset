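; BP_Pickup_Ammo is a consumable world pickup that supplies a quantity of one ammo type.
; The Construction Script sets its mesh to either a rescaled generic ammo box or a mesh selected by AmmoType.
; GetAmmoInfo returns a map of type to quantity, while GetInteractionType reports the interaction type, consumable flag and a type-based "Ammo" label.
; The event graph holds no logic, so the actor only provides data.
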(event `self.ReceiveTick`
  (params (DeltaSeconds :type "Float (single-precision)")))

(fn `GetAmmoInfo`
  (returns (`Return Value` :type Boolean) (Ammo :type "Map of /Game/RebelX_Core/Blueprints/Enums/E_WeaponTypes Enum to Integer"))
  (return true (`|MakeMap` (`self.AmmoType`) (`self.AmmoQuantity`))))

(fn `GetInteractionType`
  (returns (`Return Value` :type Boolean) (InteractionType :type "/Game/RebelX_Core/Blueprints/Enums/E_InteractionTyoes Enum") (Consumeable :type Boolean) (InteractionMessage :type Text) (IconBrush :type "SlateBrush Structure"))
  (return true "NewEnumerator1" true (`|FormatText` "{Type} Ammo" (`|GetEnumeratorNameAsString` (`self.AmmoType`)))))

(fn `UserConstructionScript`
  (bind _ammomesh (`self.AmmoMesh`))
  (if (`self.UseAmmoBoxMesh`)
    (`StaticMeshComponent.SetStaticMesh` _ammomesh "/Game/RebelX_Core/Props/Weapons/Ammo/SM_Weapons_Ammo_Box.SM_Weapons_Ammo_Box")
    (`SceneComponent.SetWorldScale3D` _ammomesh (`KismetMathLibrary.MakeVector` 0.25 0.5 0.25))
    (else
      (`StaticMeshComponent.SetStaticMesh` (`self.AmmoMesh`) (select `/Game/RebelX_Core/Blueprints/Enums/E_WeaponTypes` (`self.AmmoType`) :`NewEnumerator0` "/Game/RebelX_Core/Props/Weapons/Ammo/SM_Weapons_Ammo_Pistols.SM_Weapons_Ammo_Pistols" :`NewEnumerator7` "/Game/RebelX_Core/Props/Weapons/Ammo/SM_Weapons_Ammo_Revolvers.SM_Weapons_Ammo_Revolvers" :`NewEnumerator3` "/Game/RebelX_Core/Props/Weapons/Ammo/SM_Weapons_Ammo_Rifles.SM_Weapons_Ammo_Rifles" :`NewEnumerator6` "/Game/RebelX_Core/Props/Weapons/Ammo/SM_Weapons_Ammo_LMGs.SM_Weapons_Ammo_LMGs" :`NewEnumerator1` "/Game/RebelX_Core/Props/Weapons/Ammo/SM_Weapons_Ammo_SMGs.SM_Weapons_Ammo_SMGs" :`NewEnumerator2` "/Game/RebelX_Core/Props/Weapons/Ammo/SM_Weapons_Ammo_Shotguns.SM_Weapons_Ammo_Shotguns" :`NewEnumerator4` "/Game/RebelX_Core/Props/Weapons/Ammo/SM_Weapons_Ammo_Snipers.SM_Weapons_Ammo_Snipers" :`NewEnumerator5` "/Game/RebelX_Core/Props/Weapons/Ammo/SM_Weapons_Ammo_Launchers_Grenade.SM_Weapons_Ammo_Launchers_Grenade" :!type "StaticMesh Object Reference")))))