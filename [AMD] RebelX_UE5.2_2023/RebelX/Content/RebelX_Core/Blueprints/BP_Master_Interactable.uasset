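; BP_Master_Interactable is a base actor for interactable objects, as its name and stub functions suggest.
; Its getters for interaction type, ammo, health, weapon and scene info all return false, with placeholder outputs where present, such as an empty message and zero health.
; AttemptConsumeInteractable destroys the actor without checking the consumable flag, and the construction script is empty.
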(event `/Game/RebelX_Core/Blueprints/Interfaces/BPI_Interactables.AttemptConsumeInteractable`
  (`self.K2_DestroyActor`))

(fn `GetAmmoInfo`
  (returns (`Return Value` :type Boolean) (Ammo :type "Map of /Game/RebelX_Core/Blueprints/Enums/E_WeaponTypes Enum to Integer"))
  (return false))

(fn `GetHealthInfo`
  (returns (`Return Value` :type Boolean) (Health :type "Float (double-precision)"))
  (return false 0.0))

(fn `GetInteractionType`
  (returns (`Return Value` :type Boolean) (InteractionType :type "/Game/RebelX_Core/Blueprints/Enums/E_InteractionTyoes Enum") (Consumeable :type Boolean) (InteractionMessage :type Text) (IconBrush :type "SlateBrush Structure"))
  (return false "NewEnumerator2" false ""))

(fn `GetSceneInfo`
  (returns (`Return Value` :type Boolean))
  (return false))

(fn `GetWeaponInfo`
  (returns (`Return Value` :type Boolean) (`Weapon Data` :type "/Game/RebelX_Core/Blueprints/Structs/S_Data_Weapon Structure"))
  (return false))

(fn `UserConstructionScript`)