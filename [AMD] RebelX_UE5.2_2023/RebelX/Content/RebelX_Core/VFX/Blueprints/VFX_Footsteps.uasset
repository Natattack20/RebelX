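; Short-lived footstep effect actor that plays a surface-dependent sound, with no visual logic in its graphs.
; The construction script assigns the sound asset and maps the hit's physical material surface type to an integer "SurfaceType" audio parameter, with several surfaces sharing an index.
; BeginPlay starts the audio, and the actor destroys itself when playback finishes.
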(event `self.ReceiveBeginPlay`
  (`AudioComponent.Play` (`self.Audio`) 0.0))

(event `self.Audio.OnAudioFinished`
  (`self.K2_DestroyActor`))

(fn `UserConstructionScript`
  (bind _audio (`self.Audio`))
  (`AudioComponent.SetSound` _audio (`self.SoundAsset`))
  (`AudioParameterControllerInterface.SetIntParameter` _audio "SurfaceType" (select `EPhysicalSurface` (`PhysicalMaterial.SurfaceType` (`.PhysMat` (`GameplayStatics.BreakHitResult` (`self.Hit`)))) :`SurfaceType1` 1 :`SurfaceType2` 2 :`SurfaceType3` 3 :`SurfaceType4` 4 :`SurfaceType5` 1 :`SurfaceType7` 2 :`SurfaceType8` 5 :`SurfaceType11` 3 :`SurfaceType14` 6 :`SurfaceType16` 7 :`SurfaceType19` 8 :`SurfaceType20` 9 :`SurfaceType22` 10 :`SurfaceType23` 11 :`SurfaceType24` 4)))