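; Master impact effect actor that pairs a sound, Niagara effect and decal for a hit on a given SurfaceType, using bullet-hit cues.
; The construction script assigns all three components, picking sound and effect through per-surface Select lookups.
; Leaves randomize their effect, though the fourth variant is out of range; Plaster and Rock have no effect assigned.
; The decal is always the scorch material, and the event graph runs no logic.
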(event `self.ReceiveBeginPlay`)

(fn `GetAudioAsset`
  (returns (ReturnValue :type "SoundBase Object Reference"))
  (return (select `EPhysicalSurface` (`self.SurfaceType`) :`SurfaceType_Default` "/Game/RebelX_Core/Audio/Impacts/SC_Bullet_Hit_Dirt.SC_Bullet_Hit_Dirt" :`SurfaceType1` "/Game/RebelX_Core/Audio/Impacts/SC_Bullet_Hit_Dirt.SC_Bullet_Hit_Dirt" :`SurfaceType2` "/Game/RebelX_Core/Audio/Impacts/SC_Bullet_Hit_Body.SC_Bullet_Hit_Body" :`SurfaceType3` "/Game/RebelX_Core/Audio/Impacts/SC_Bullet_Hit_Dirt.SC_Bullet_Hit_Dirt" :`SurfaceType4` "/Game/RebelX_Core/Audio/Impacts/SC_Bullet_Hit_Dirt.SC_Bullet_Hit_Dirt" :`SurfaceType5` "/Game/RebelX_Core/Audio/Impacts/SC_Bullet_Hit_Dirt.SC_Bullet_Hit_Dirt" :`SurfaceType6` "/Game/RebelX_Core/Audio/Impacts/SC_Bullet_Hit_Dirt.SC_Bullet_Hit_Dirt" :`SurfaceType7` "/Game/RebelX_Core/Audio/Impacts/SC_Bullet_Hit_Dirt.SC_Bullet_Hit_Dirt" :`SurfaceType8` "/Game/RebelX_Core/Audio/Impacts/SC_Bullet_Hit_Dirt.SC_Bullet_Hit_Dirt" :`SurfaceType9` "/Game/RebelX_Core/Audio/Impacts/SC_Bullet_Hit_Metal.SC_Bullet_Hit_Metal" :`SurfaceType10` "/Game/RebelX_Core/Audio/Impacts/SC_Bullet_Hit_Glass.SC_Bullet_Hit_Glass" :`SurfaceType11` "/Game/RebelX_Core/Audio/Impacts/SC_Bullet_Hit_Dirt.SC_Bullet_Hit_Dirt" :`SurfaceType12` "/Game/RebelX_Core/Audio/Impacts/SC_Bullet_Hit_Glass_bottle_Whizz.SC_Bullet_Hit_Glass_bottle_Whizz" :`SurfaceType13` "/Game/RebelX_Core/Audio/Impacts/SC_Bullet_Hit_Dirt.SC_Bullet_Hit_Dirt" :`SurfaceType14` "/Game/RebelX_Core/Audio/Impacts/SC_Bullet_Hit_Metal.SC_Bullet_Hit_Metal" :`SurfaceType15` "/Game/RebelX_Core/Audio/Impacts/SC_Bullet_Hit_Dirt.SC_Bullet_Hit_Dirt" :`SurfaceType16` "/Game/RebelX_Core/Audio/Impacts/SC_Bullet_Hit_Dirt.SC_Bullet_Hit_Dirt" :`SurfaceType17` "/Game/RebelX_Core/Audio/Impacts/SC_Bullet_Hit_Dirt.SC_Bullet_Hit_Dirt" :`SurfaceType18` "/Game/RebelX_Core/Audio/Impacts/SC_Bullet_Hit_Dirt.SC_Bullet_Hit_Dirt" :`SurfaceType19` "/Game/RebelX_Core/Audio/Impacts/SC_Bullet_Hit_Dirt.SC_Bullet_Hit_Dirt" :`SurfaceType20` "/Game/RebelX_Core/Audio/Impacts/SC_Bullet_Hit_Dirt.SC_Bullet_Hit_Dirt" :`SurfaceType21` "/Game/RebelX_Core/Audio/Impacts/SC_Bullet_Hit_Dirt.SC_Bullet_Hit_Dirt" :`SurfaceType22` "/Game/RebelX_Core/Audio/Impacts/SC_Bullet_Hit_Water.SC_Bullet_Hit_Water" :`SurfaceType23` "/Game/RebelX_Core/Audio/Impacts/SC_Bullet_Hit_Wood_Whizz.SC_Bullet_Hit_Wood_Whizz" :`SurfaceType24` "/Game/RebelX_Core/Audio/Impacts/SC_Bullet_Hit_Dirt.SC_Bullet_Hit_Dirt" :!type "SoundBase Object Reference")))

(fn `GetDecalAsset`
  (returns (ReturnValue :type "MaterialInterface Object Reference"))
  (return "/Game/RebelX_Core/VFX/Materials/Decals/MI_Scorch.MI_Scorch"))

(fn `GetSystemAsset`
  (returns (ReturnValue :type "NiagaraSystem Object Reference"))
  (return (select `EPhysicalSurface` (`self.SurfaceType`) :`SurfaceType_Default` "/Game/RebelX_Core/VFX/Impacts/Systems/NS_Impact_Dirt.NS_Impact_Dirt" :`SurfaceType1` "/Game/RebelX_Core/VFX/Impacts/Systems/NS_Impact_Asphalt.NS_Impact_Asphalt" :`SurfaceType2` "/Game/RebelX_Core/VFX/Impacts/Systems/NS_Impact_Blood.NS_Impact_Blood" :`SurfaceType3` "/Game/RebelX_Core/VFX/Impacts/Systems/NS_Impact_Brick.NS_Impact_Brick" :`SurfaceType4` "/Game/RebelX_Core/VFX/Impacts/Systems/NS_Impact_Cardboard.NS_Impact_Cardboard" :`SurfaceType5` "/Game/RebelX_Core/VFX/Impacts/Systems/NS_Impact_Carpet.NS_Impact_Carpet" :`SurfaceType6` "/Game/RebelX_Core/VFX/Impacts/Systems/NS_Impact_Cloth.NS_Impact_Cloth" :`SurfaceType7` "/Game/RebelX_Core/VFX/Impacts/Systems/NS_Impact_Concrete.NS_Impact_Concrete" :`SurfaceType8` "/Game/RebelX_Core/VFX/Impacts/Systems/NS_Impact_Dirt.NS_Impact_Dirt" :`SurfaceType9` "/Game/RebelX_Core/VFX/Impacts/Systems/NS_Impact_Electronics.NS_Impact_Electronics" :`SurfaceType10` "/Game/RebelX_Core/VFX/Impacts/Systems/NS_Impact_Glass.NS_Impact_Glass" :`SurfaceType11` "/Game/RebelX_Core/VFX/Impacts/Systems/NS_Impact_Grass.NS_Impact_Grass" :`SurfaceType12` "/Game/RebelX_Core/VFX/Impacts/Systems/NS_Impact_Water.NS_Impact_Water" :`SurfaceType13` (select `int` (`KismetMathLibrary.RandomIntegerInRange` 0 2) :`0` "/Game/RebelX_Core/VFX/Impacts/Systems/NS_Impact_Leaves1.NS_Impact_Leaves1" :`1` "/Game/RebelX_Core/VFX/Impacts/Systems/NS_Impact_Leaves_01.NS_Impact_Leaves_01" :`2` "/Game/RebelX_Core/VFX/Impacts/Systems/NS_Impact_Leaves_02.NS_Impact_Leaves_02" :`3` "/Game/RebelX_Core/VFX/Impacts/Systems/NS_Impact_Leaves_03.NS_Impact_Leaves_03" :!type "NiagaraSystem Object Reference") :`SurfaceType14` "/Game/RebelX_Core/VFX/Impacts/Systems/NS_Impact_Metal.NS_Impact_Metal" :`SurfaceType16` "/Game/RebelX_Core/VFX/Impacts/Systems/NS_Impact_Plastic.NS_Impact_Plastic" :`SurfaceType18` "/Game/RebelX_Core/VFX/Impacts/Systems/NS_Impact_Plastic.NS_Impact_Plastic" :`SurfaceType19` "/Game/RebelX_Core/VFX/Impacts/Systems/NS_Impact_Sand.NS_Impact_Sand" :`SurfaceType20` "/Game/RebelX_Core/VFX/Impacts/Systems/NS_Impact_Snow.NS_Impact_Snow" :`SurfaceType21` "/Game/RebelX_Core/VFX/Impacts/Systems/NS_Impact_Tile.NS_Impact_Tile" :`SurfaceType22` "/Game/RebelX_Core/VFX/Impacts/Systems/NS_Impact_Water.NS_Impact_Water" :`SurfaceType23` "/Game/RebelX_Core/VFX/Impacts/Systems/NS_Impact_Wood.NS_Impact_Wood" :`SurfaceType24` "/Game/RebelX_Core/VFX/Impacts/Systems/NS_Impact_Dirt.NS_Impact_Dirt")))

(fn `UserConstructionScript`
  (`|ExecutionSequence`
    (:`then_0`
      (bind _returnvalue (`self.GetAudioAsset`))
      (`AudioComponent.SetSound` (`self.Audio`) _returnvalue))
    (:`then_1`
      (bind _returnvalue_2 (`self.GetSystemAsset`))
      (`NiagaraComponent.SetAsset` (`self.Niagara`) _returnvalue_2 true))
    (:`then_2`
      (bind _returnvalue_3 (`self.GetDecalAsset`))
      (`DecalComponent.SetDecalMaterial` (`self.Decal`) _returnvalue_3))))