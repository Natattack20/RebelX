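; BP_IconRenderer is a utility that renders the mesh in its StaticMesh component into an icon texture.
; On BeginPlay or through RenderIcons, it triggers a scene capture and converts ActiveRenderTarget into a static texture with editor-only RenderTargetCreateStaticTexture2DEditorOnly.
; It also exports that texture as a PNG to the project's Content folder, naming it after the mesh with SM_ replaced by UIT_.
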(event `self.ReceiveBeginPlay`
  (`self.StartRender`))

(event `StartRender`
  (bind _returnvalue (`KismetStringLibrary.Concat_StrStr` (`KismetStringLibrary.Replace` (`KismetSystemLibrary.GetDisplayName` (`StaticMeshComponent.StaticMesh` (`self.StaticMesh`))) "SM_" "UIT_") ".png"))
  (`SceneCaptureComponent2D.CaptureScene` (`self.SceneCaptureComponent2D`))
  (bind _returnvalue_2 (`KismetRenderingLibrary.RenderTargetCreateStaticTexture2DEditorOnly` (`self.ActiveRenderTarget`) _returnvalue "TC_EditorIcon"))
  (`ImageWriteBlueprintLibrary.ExportToDisk` _returnvalue_2 (`KismetStringLibrary.Concat_StrStr` (`KismetSystemLibrary.GetProjectDirectory`) "Content/" _returnvalue) (make `ImageWriteOptions` "PNG")))

(fn `RenderIcons`
  (`self.StartRender`))

(fn `UserConstructionScript`)