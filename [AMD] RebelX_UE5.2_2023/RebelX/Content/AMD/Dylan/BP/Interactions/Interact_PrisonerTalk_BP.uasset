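; Interactable actor, named for talking to a prisoner, that implements the interaction query and event functions.
; It reports itself as a consumable interaction with a fixed type and a variable prompt message, and supplies no HUD or scene info.
; Consuming it destroys the actor after a short delay, while scene activation only blanks the prompt message.
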(event `/Game/RebelX_Core/Blueprints/Interfaces/BPI_Interactables.AttemptConsumeInteractable`
  (`KismetSystemLibrary.Delay` 0.2)
  (`self.K2_DestroyActor`))

(event `/Game/RebelX_Core/Blueprints/Interfaces/BPI_Interactables.ActivateSceneObject`
  (set `self.Interaction Message` ""))

(fn `GetAttachedHUD`
  (returns (`AsHUD Rebel X` :type "/Game/RebelX_Core/Blueprints/HUD_RebelX Object Reference"))
  (return null))

(fn `GetInteractionType`
  (returns (`Return Value` :type Boolean) (InteractionType :type "/Game/RebelX_Core/Blueprints/Enums/E_InteractionTyoes Enum") (Consumeable :type Boolean) (InteractionMessage :type Text) (IconBrush :type "SlateBrush Structure"))
  (return true "NewEnumerator2" true (`self.Interaction Message`)))

(fn `GetSceneInfo`
  (returns (`Return Value` :type Boolean))
  (return false))

(fn `UserConstructionScript`
  (`parent.UserConstructionScript`))