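; Alarm light actor that spins and flashes a cylinder mesh from the moment play begins.
; A timeline started on BeginPlay drives the cylinder's yaw.
; Each timeline update also feeds a DoOnce that sets a red material, switches to concrete after a short delay, then resets after a second delay, so the blink repeats while the timeline updates.
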(event `self.ReceiveBeginPlay`
  (bind _cylinder (`self.Cylinder`))
  (bind (_direction _newtrack_0) (`Timeline|Roatating Lights` :!via `PlayFromStart`)
    (:`Update`
      (`SceneComponent.K2_SetRelativeRotation` (`self.Cylinder`) (`KismetMathLibrary.MakeRotator` 0.0 0.0 _newtrack_0) false false)
      (`/Engine/EditorBlueprintResources/StandardMacros.DoOnce` false :!label _label
        (:`Completed`
          (`|ExecutionSequence`
            (:`then_0`
              (`PrimitiveComponent.SetMaterial` _cylinder 0 "/Game/AMD/Dylan/Mats/MyMats/M_Red.M_Red"))
            (:`then_1`
              (`KismetSystemLibrary.Delay` 0.5)
              (`PrimitiveComponent.SetMaterial` _cylinder 0 "/Game/RebelX_Core/Environment/Materials/Concrete/MI_Concrete.MI_Concrete")
              (`KismetSystemLibrary.Delay` 0.5)
              (goto _label :!via `Reset`))))))))

(fn `UserConstructionScript`)