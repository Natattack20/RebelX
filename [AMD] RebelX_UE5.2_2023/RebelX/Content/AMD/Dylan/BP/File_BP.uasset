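; Interactable gate key pickup for level 3, collected with an 'E' prompt and marked consumable.
; Interface-style getters report the interaction type and message, while scene, ammo, health and weapon queries return false.
; On BeginPlay it caches the Player_RebelX character.
; ActivateSceneObject updates the HUD objective to unlock the gate toward the yard and sets the player's LVL3GateKey flag.
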(event `self.ReceiveBeginPlay`
  (bind _asplayer_rebel_x (cast `/Game/RebelX_Core/Blueprints/Player_RebelX` (`GameplayStatics.GetPlayerCharacter` 0)))
  (set `self.As Player Rebel X` _asplayer_rebel_x))

(event `/Game/RebelX_Core/Blueprints/Interfaces/BPI_Interactables.ActivateSceneObject`
  (message `/Game/RebelX_Core/Blueprints/Interfaces/BPI_HUD.UpdateObjective` (`PlayerController.GetHUD` (`GameplayStatics.GetPlayerController` 0)) "The Key!" "Unlock the gate and proceed to the yard.")
  (set `/Game/RebelX_Core/Blueprints/Player_RebelX.LVL3_GateKey` true (`self.As Player Rebel X`)))

(fn `GetAmmoInfo`
  (returns (`Return Value` :type Boolean) (Ammo :type "Map of /Game/RebelX_Core/Blueprints/Enums/E_WeaponTypes Enum to Integer"))
  (return false))

(fn `GetHealthInfo`
  (returns (`Return Value` :type Boolean) (Health :type "Float (double-precision)"))
  (return false 0.0))

(fn `GetInteractionType`
  (returns (`Return Value` :type Boolean) (InteractionType :type "/Game/RebelX_Core/Blueprints/Enums/E_InteractionTyoes Enum") (Consumeable :type Boolean) (InteractionMessage :type Text) (IconBrush :type "SlateBrush Structure"))
  (return true "NewEnumerator2" true "Press 'E' to collect gate key"))

(fn `GetSceneInfo`
  (returns (`Return Value` :type Boolean))
  (return false))

(fn `GetWeaponInfo`
  (returns (`Return Value` :type Boolean) (`Weapon Data` :type "/Game/RebelX_Core/Blueprints/Structs/S_Data_Weapon Structure"))
  (return false))

(fn `UserConstructionScript`
  (`parent.UserConstructionScript`))