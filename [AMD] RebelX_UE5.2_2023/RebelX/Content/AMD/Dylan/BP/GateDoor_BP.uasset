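; GateDoor_BP is an interactable Level 3 gate that the player unlocks with a key.
; On BeginPlay it caches the Player_RebelX character, then reports an unlock prompt through GetInteractionType, using the player's key flag as Consumeable.
; ActivateSceneObject flags the gate interaction on the player, and sets LVL3GateDoor only if the key is held.
; It only writes player state and moves no door itself; the other info getters are stubs returning false.
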(event `self.ReceiveBeginPlay`
  (bind _asplayer_rebel_x (cast `/Game/RebelX_Core/Blueprints/Player_RebelX` (`GameplayStatics.GetPlayerCharacter` 0)))
  (set `self.As Player Rebel X` _asplayer_rebel_x))

(event `/Game/RebelX_Core/Blueprints/Interfaces/BPI_Interactables.ActivateSceneObject`
  (bind _as_player_rebel_x (`self.As Player Rebel X`))
  (set `/Game/RebelX_Core/Blueprints/Player_RebelX.LVL3_IntGate` true _as_player_rebel_x)
  (if (`/Game/RebelX_Core/Blueprints/Player_RebelX.LVL3_GateKey` _as_player_rebel_x)
    (set `/Game/RebelX_Core/Blueprints/Player_RebelX.LVL3_GateDoor` true _as_player_rebel_x)))

(fn `GetAmmoInfo`
  (returns (`Return Value` :type Boolean) (Ammo :type "Map of /Game/RebelX_Core/Blueprints/Enums/E_WeaponTypes Enum to Integer"))
  (return false))

(fn `GetHealthInfo`
  (returns (`Return Value` :type Boolean) (Health :type "Float (double-precision)"))
  (return false 0.0))

(fn `GetInteractionType`
  (returns (`Return Value` :type Boolean) (InteractionType :type "/Game/RebelX_Core/Blueprints/Enums/E_InteractionTyoes Enum") (Consumeable :type Boolean) (InteractionMessage :type Text) (IconBrush :type "SlateBrush Structure"))
  (return true "NewEnumerator2" (`/Game/RebelX_Core/Blueprints/Player_RebelX.LVL3_GateKey` (`self.As Player Rebel X`)) "Press 'E' to Unlock gate"))

(fn `GetSceneInfo`
  (returns (`Return Value` :type Boolean))
  (return false))

(fn `GetWeaponInfo`
  (returns (`Return Value` :type Boolean) (`Weapon Data` :type "/Game/RebelX_Core/Blueprints/Structs/S_Data_Weapon Structure"))
  (return false))

(fn `UserConstructionScript`
  (`parent.UserConstructionScript`))