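; Interactable main gates switch for level 3 that flags the player's button progress, updates the HUD objective and triggers an ambush.
; Activation through the scene-object interaction interface clears the prompt, activates two spawners and applies damage to itself from the player.
; A DoOnce then dips the static mesh slightly and raises it after a delay, like a button press.
; The other interface getters for scene, ammo, health and weapon info return false.
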(event `self.ReceiveBeginPlay`
  (bind _asplayer_rebel_x (cast `/Game/RebelX_Core/Blueprints/Player_RebelX` (`GameplayStatics.GetPlayerCharacter` 0)))
  (bind _output_get (set `self.As Player Rebel X` _asplayer_rebel_x)))

(event `/Game/RebelX_Core/Blueprints/Interfaces/BPI_Interactables.ActivateSceneObject`
  (bind _staticmesh (`self.StaticMesh`))
  (bind _staticmesh_2 (`self.StaticMesh`))
  (bind (_returnvalue_x _returnvalue_y _returnvalue_z) (`KismetMathLibrary.BreakVector` (`SceneComponent.K2_GetComponentLocation` _staticmesh_2)))
  (bind (_returnvalue_x_2 _returnvalue_y_2 _returnvalue_z_2) (`KismetMathLibrary.BreakVector` (`SceneComponent.K2_GetComponentLocation` _staticmesh)))
  (set `/Game/RebelX_Core/Blueprints/Player_RebelX.LVL3_HasntPressedButton` true (`self.As Player Rebel X`))
  (message `/Game/RebelX_Core/Blueprints/Interfaces/BPI_HUD.UpdateObjective` (`PlayerController.GetHUD` (`GameplayStatics.GetPlayerController` 0)) "Nearly out!" "Go the gate is open but it looks like there prepared!")
  (set `self.Interaction Message` "")
  (`/Game/RebelX_Core/Blueprints/Gameplay/BP_Spawner_Droid.ActivateSpawner` (`self.Spawner`))
  (`/Game/RebelX_Core/Blueprints/Gameplay/BP_Spawner_Droid.ActivateSpawner` (`self.Spawner_0`))
  (`GameplayStatics.ApplyDamage` self 5.0 null (stale `self.ReceiveBeginPlay` _output_get))
  (`/Engine/EditorBlueprintResources/StandardMacros.DoOnce` false
    (:`Completed`
      (`SceneComponent.K2_SetWorldLocation` _staticmesh_2 (`KismetMathLibrary.MakeVector` _returnvalue_x _returnvalue_y (- _returnvalue_z 5.0)) false false)
      (`KismetSystemLibrary.Delay` 2.0)
      (`SceneComponent.K2_SetWorldLocation` _staticmesh (`KismetMathLibrary.MakeVector` _returnvalue_x_2 _returnvalue_y_2 (+ _returnvalue_z_2 5.0)) false false))))

(fn `GetAmmoInfo`
  (returns (`Return Value` :type Boolean) (Ammo :type "Map of /Game/RebelX_Core/Blueprints/Enums/E_WeaponTypes Enum to Integer"))
  (return false))

(fn `GetHealthInfo`
  (returns (`Return Value` :type Boolean) (Health :type "Float (double-precision)"))
  (return false 0.0))

(fn `GetInteractionType`
  (returns (`Return Value` :type Boolean) (InteractionType :type "/Game/RebelX_Core/Blueprints/Enums/E_InteractionTyoes Enum") (Consumeable :type Boolean) (InteractionMessage :type Text) (IconBrush :type "SlateBrush Structure"))
  (return true "NewEnumerator2" false (`self.Interaction Message`)))

(fn `GetSceneInfo`
  (returns (`Return Value` :type Boolean))
  (return false))

(fn `GetWeaponInfo`
  (returns (`Return Value` :type Boolean) (`Weapon Data` :type "/Game/RebelX_Core/Blueprints/Structs/S_Data_Weapon Structure"))
  (return false))

(fn `UserConstructionScript`
  (`parent.UserConstructionScript`))