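; TowerWall_BP is a tower wall actor that plays a one-time explosion sequence when its SucessValve event is called.
; BeginPlay caches the Rebel X player, and SucessValve triggers that player's ValveFocusEvent behind a DoOnce.
; It then activates three NIExpo effects in a short staggered sequence, each paired with a world camera shake centered on the player's mesh.
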(event `self.ReceiveBeginPlay`
  (bind _asplayer_rebel_x (cast `/Game/RebelX_Core/Blueprints/Player_RebelX` (`GameplayStatics.GetPlayerCharacter` 0)))
  (set `self.As Player Rebel X` _asplayer_rebel_x))

(event `Sucess Valve`
  (bind _returnvalue (`SceneComponent.K2_GetComponentLocation` (`Character.Mesh` (`self.As Player Rebel X`))))
  (`/Engine/EditorBlueprintResources/StandardMacros.DoOnce` false
    (:`Completed`
      (`/Game/RebelX_Core/Blueprints/Player_RebelX.Valve Focus Event` (`self.As Player Rebel X`))
      (`ActorComponent.Activate` (`self.NI_Expo1`) false)
      (`GameplayStatics.PlayWorldCameraShake` "/Game/AMD/Dylan/BP/Cam_Shake.Cam_Shake_C" _returnvalue 0.0 500.0)
      (`KismetSystemLibrary.Delay` 0.2)
      (`GameplayStatics.PlayWorldCameraShake` "/Game/AMD/Dylan/BP/Cam_Shake.Cam_Shake_C" _returnvalue 0.0 500.0)
      (`ActorComponent.Activate` (`self.NI_Expo2`) false)
      (`KismetSystemLibrary.Delay` 0.2)
      (`GameplayStatics.PlayWorldCameraShake` "/Game/AMD/Dylan/BP/Cam_Shake.Cam_Shake_C" _returnvalue 0.0 500.0)
      (`ActorComponent.Activate` (`self.NI_Expo3`) false))))

(fn `UserConstructionScript`)