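; Interactable gate that the player opens with the level 3 gate key on Player_RebelX.
; Activation drops the lock with physics and swings the right door by timeline, whose first update starts a second timeline for the left door.
; The left door's update removes the widget once, plays a sound and clears the key.
; If the player's level 1 valve flag is set, it then calls SucessValve on TowerWall_BP after a short delay.
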(event `self.ReceiveBeginPlay`
  (bind _asplayer_rebel_x (cast `/Game/RebelX_Core/Blueprints/Player_RebelX` (`GameplayStatics.GetPlayerCharacter` 0)))
  (set `self.As Player Rebel X` _asplayer_rebel_x))

(event `/Game/RebelX_Core/Blueprints/Interfaces/BPI_Interactables.ActivateSceneObject`
  (bind _widget (`self.Widget`))
  (bind _l (`self.L`))
  (bind _r (`self.R`))
  (bind _lock (`self.Lock`))
  (bind (_returnvalue_roll _returnvalue_pitch) (`KismetMathLibrary.BreakRotator` (`SceneComponent.K2_GetComponentRotation` _r)))
  (bind (_returnvalue_roll_2 _returnvalue_pitch_2) (`KismetMathLibrary.BreakRotator` (`SceneComponent.K2_GetComponentRotation` _l)))
  (if (`/Game/RebelX_Core/Blueprints/Player_RebelX.LVL3_GateKey` (`self.As Player Rebel X`))
    (`PrimitiveComponent.SetSimulatePhysics` _lock true)
    (`PrimitiveComponent.SetCollisionEnabled` _lock "ProbeOnly")
    (bind (_direction _newtrack_0) (`Timeline|GateDoors`)
      (:`Update`
        (`SceneComponent.K2_SetWorldRotation` _r (`KismetMathLibrary.MakeRotator` _returnvalue_roll _returnvalue_pitch (`KismetMathLibrary.Lerp` 0.0 140.0 _newtrack_0)) false false)
        (`/Engine/EditorBlueprintResources/StandardMacros.DoOnce` false
          (:`Completed`
            (bind (_direction_2 _newtrack_0_2) (`Timeline|Timeline`)
              (:`Update`
                (`SceneComponent.K2_SetWorldRotation` _l (`KismetMathLibrary.MakeRotator` _returnvalue_roll_2 _returnvalue_pitch_2 (`KismetMathLibrary.Lerp` 0.0 -110.0 _newtrack_0_2)) false false)
                (`/Engine/EditorBlueprintResources/StandardMacros.IsValid` _widget
                  (:`Is Valid`
                    (`ActorComponent.K2_DestroyComponent` _widget)
                    (`GameplayStatics.PlaySound2D` "/Game/AMD/Dylan/Audio/Dil_Gary_Todd_Gary_Todd_00001.Dil_Gary_Todd_Gary_Todd_00001" 1.0 1.0 0.0 null null)
                    (set `/Game/RebelX_Core/Blueprints/Player_RebelX.LVL3_GateKey` false (`self.As Player Rebel X`))
                    (`GameplayStatics.GetActorOfClass` "/Game/AMD/Dylan/BP/TowerWall_BP.TowerWall_BP_C")
                    (if (`/Game/RebelX_Core/Blueprints/Player_RebelX.LV1_Valve_Sucess` (`self.As Player Rebel X`))
                      (bind _returnvalue (`GameplayStatics.GetActorOfClass` "/Game/AMD/Dylan/BP/TowerWall_BP.TowerWall_BP_C"))
                      (`KismetSystemLibrary.Delay` 0.5)
                      (`/Game/AMD/Dylan/BP/TowerWall_BP.Sucess Valve` _returnvalue))))))))))))

(fn `GetInteractionType`
  (returns (`Return Value` :type Boolean) (InteractionType :type "/Game/RebelX_Core/Blueprints/Enums/E_InteractionTyoes Enum") (Consumeable :type Boolean) (InteractionMessage :type Text) (IconBrush :type "SlateBrush Structure"))
  (return true "NewEnumerator2" false "Press 'E' to open gate"))

(fn `UserConstructionScript`
  (`parent.UserConstructionScript`))