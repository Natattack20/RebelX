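; Spotlight actor that tests line of sight to the Player_RebelX player, apparently as prototype detection.
; BeginPlay caches the player; each Tick line-traces on Visibility from the light to the player's mesh, printing "Not Seen" on a blocking hit, otherwise "Spotted".
; The check ignores the light's direction and cone angle.
; An unconnected timeline sphere trace and unused cone and distance nodes remain, and detection only produces debug output.
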(event `self.ReceiveBeginPlay`
  (bind _asplayer_rebel_x (cast `/Game/RebelX_Core/Blueprints/Player_RebelX` (`GameplayStatics.GetPlayerCharacter` 0)))
  (set `self.As Player Rebel X` _asplayer_rebel_x))

(event `self.ReceiveTick`
  (params (DeltaSeconds :type "Float (single-precision)"))
  (bind _outhit (`KismetSystemLibrary.LineTraceSingle` :`Start` (`SceneComponent.K2_GetComponentLocation` (`self.SpotLight`)) :`End` (`SceneComponent.K2_GetComponentLocation` (`Character.Mesh` (`self.As Player Rebel X`))) :`TraceChannel` "TraceTypeQuery1" :`DrawDebugType` "ForDuration" :`DrawTime` 0.1))
  (if (`GameplayStatics.BreakHitResult` _outhit)
    (`KismetSystemLibrary.PrintString` "Not Seen")
    (else
      (`KismetSystemLibrary.PrintString` "Spotted"))))

(fn `UserConstructionScript`)