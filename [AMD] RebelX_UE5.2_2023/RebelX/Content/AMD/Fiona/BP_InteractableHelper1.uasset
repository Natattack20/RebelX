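; Interactable helper actor that offers a reusable "Talk?" prompt and toggles the UI_WeaponCode widget when activated.
; GetInteractionType supplies the interaction type, message and non-consumable flag, while ActivateSceneObject flips an Open flag to create or remove the widget.
; Closing restores game-only input; opening leaves the input mode unchanged.
; BeginPlay caches the Player_RebelX character, though these graphs never use it afterward.
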(event `self.ReceiveBeginPlay`
  (bind _asplayer_rebel_x (cast `/Game/RebelX_Core/Blueprints/Player_RebelX` (`GameplayStatics.GetPlayerCharacter` 0)))
  (set `self.As Player Rebel X` _asplayer_rebel_x))

(event `/Game/RebelX_Core/Blueprints/Interfaces/BPI_Interactables.ActivateSceneObject`
  (if (`self.Open`)
    (set `self.Open` false)
    (`WidgetBlueprintLibrary.SetInputMode_GameOnly` (`GameplayStatics.GetPlayerController` 0))
    (`Widget.RemoveFromParent` (stale _returnvalue))
    (else
      (set `self.Open` true)
      (bind _returnvalue (`|CreateWidget` "/Game/AMD/Fiona/UI_WeaponCode.UI_WeaponCode_C" null self))
      (`UserWidget.AddToViewport` _returnvalue 0))))

(fn `GetInteractionType`
  (returns (`Return Value` :type Boolean) (InteractionType :type "/Game/RebelX_Core/Blueprints/Enums/E_InteractionTyoes Enum") (Consumeable :type Boolean) (InteractionMessage :type Text) (IconBrush :type "SlateBrush Structure"))
  (return true "NewEnumerator2" false "Talk?"))

(fn `UserConstructionScript`
  (`parent.UserConstructionScript`))