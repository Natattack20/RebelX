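; BP_ValveCode is an interactable scene object that shows a valve code UI when the player inspects it.
; Activating it toggles an Open flag, either creating UI_ValveCode and adding it to the viewport or removing it and restoring game-only input.
; Its info getters report it only as an interaction with an "Inspect?" prompt, not a weapon, ammo or health item.
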(event `/Game/RebelX_Core/Blueprints/Interfaces/BPI_Interactables.ActivateSceneObject`
  (if (`self.Open`)
    (set `self.Open` false)
    (`WidgetBlueprintLibrary.SetInputMode_GameOnly` (`GameplayStatics.GetPlayerController` 0))
    (`Widget.RemoveFromParent` (stale _returnvalue))
    (else
      (set `self.Open` true)
      (bind _returnvalue (`|CreateWidget` "/Game/AMD/Fiona/UI_ValveCode.UI_ValveCode_C" null self))
      (`UserWidget.AddToViewport` _returnvalue 0))))

(fn `GetAmmoInfo`
  (returns (`Return Value` :type Boolean) (Ammo :type "Map of /Game/RebelX_Core/Blueprints/Enums/E_WeaponTypes Enum to Integer"))
  (return false))

(fn `GetHealthInfo`
  (returns (`Return Value` :type Boolean) (Health :type "Float (double-precision)"))
  (return false 0.0))

(fn `GetInteractionType`
  (returns (`Return Value` :type Boolean) (InteractionType :type "/Game/RebelX_Core/Blueprints/Enums/E_InteractionTyoes Enum") (Consumeable :type Boolean) (InteractionMessage :type Text) (IconBrush :type "SlateBrush Structure"))
  (return true "NewEnumerator2" false "Inspect?"))

(fn `GetSceneInfo`
  (returns (`Return Value` :type Boolean))
  (return false))

(fn `GetWeaponInfo`
  (returns (`Return Value` :type Boolean) (`Weapon Data` :type "/Game/RebelX_Core/Blueprints/Structs/S_Data_Weapon Structure"))
  (return false))

(fn `UserConstructionScript`
  (`parent.UserConstructionScript`))