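; BP_InteractableHelper is a talk interactable that grants the Rebel X player the cell key.
; GetInteractionType reports a non-consumable interaction with a talk prompt.
; ActivateSceneObject sets HasCellKey on the player cached at BeginPlay, disables movement and plays a 2D audio clip.
; After a fixed delay timed in seconds rather than by audio completion, it plays a keycard unlock sound and restores walking.
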(event `self.ReceiveBeginPlay`
  (bind _asplayer_rebel_x (cast `/Game/RebelX_Core/Blueprints/Player_RebelX` (`GameplayStatics.GetPlayerCharacter` 0)))
  (set `self.As Player Rebel X` _asplayer_rebel_x))

(event `/Game/RebelX_Core/Blueprints/Interfaces/BPI_Interactables.ActivateSceneObject`
  (bind _as_player_rebel_x (`self.As Player Rebel X`))
  (bind _charactermovement (`Character.CharacterMovement` _as_player_rebel_x))
  (set `/Game/RebelX_Core/Blueprints/Player_RebelX.HasCellKey` true _as_player_rebel_x)
  (`CharacterMovementComponent.DisableMovement` _charactermovement)
  (`GameplayStatics.PlaySound2D` "/Game/AMD/Fiona/Audio/audio_12.audio_12" 1.0 1.0 0.0 null null)
  (`KismetSystemLibrary.Delay` 12.0)
  (`GameplayStatics.PlaySound2D` "/Game/RX_C_Bailey_Content/Sounds/KeycardUnlock.KeycardUnlock" 1.0 1.0 0.0 null null)
  (`CharacterMovementComponent.SetMovementMode` _charactermovement "MOVE_Walking" 0))

(fn `GetInteractionType`
  (returns (`Return Value` :type Boolean) (InteractionType :type "/Game/RebelX_Core/Blueprints/Enums/E_InteractionTyoes Enum") (Consumeable :type Boolean) (InteractionMessage :type Text) (IconBrush :type "SlateBrush Structure"))
  (return true "NewEnumerator2" false " E to \nTalk?"))

(fn `UserConstructionScript`
  (`parent.UserConstructionScript`))