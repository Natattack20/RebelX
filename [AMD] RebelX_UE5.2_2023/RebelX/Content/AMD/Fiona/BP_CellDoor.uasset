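; BP_CellDoor is an interactable cell door that opens only when the player holds the cell key.
; It caches the Player_RebelX character on BeginPlay and reports an "Open cell" interaction prompt through GetInteractionType.
; On ActivateSceneObject it checks HasCellKey, then either swings the static mesh's yaw open with a Timeline-driven lerp or shows the UI_NeedKey widget.
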(event `self.ReceiveBeginPlay`
  (bind _asplayer_rebel_x (cast `/Game/RebelX_Core/Blueprints/Player_RebelX` (`GameplayStatics.GetPlayerCharacter` 0)))
  (set `self.As Player Rebel X` _asplayer_rebel_x))

(event `/Game/RebelX_Core/Blueprints/Interfaces/BPI_Interactables.ActivateSceneObject`
  (bind _staticmesh (`self.StaticMesh`))
  (bind (_returnvalue_roll _returnvalue_pitch) (`KismetMathLibrary.BreakRotator` (`SceneComponent.K2_GetComponentRotation` _staticmesh)))
  (if (`/Game/RebelX_Core/Blueprints/Player_RebelX.HasCellKey` (`self.As Player Rebel X`))
    (bind (_direction _newtrack_0) (`Timeline|Timeline`)
      (:`Update`
        (`SceneComponent.K2_SetWorldRotation` _staticmesh (`KismetMathLibrary.MakeRotator` _returnvalue_roll _returnvalue_pitch (`KismetMathLibrary.Lerp` -90.0 -30.0 _newtrack_0)) false false)))
    (else
      (bind _returnvalue (`|CreateWidget` "/Game/AMD/Fiona/UI_NeedKey.UI_NeedKey_C"))
      (`UserWidget.AddToViewport` _returnvalue 0))))

(fn `GetInteractionType`
  (returns (`Return Value` :type Boolean) (InteractionType :type "/Game/RebelX_Core/Blueprints/Enums/E_InteractionTyoes Enum") (Consumeable :type Boolean) (InteractionMessage :type Text) (IconBrush :type "SlateBrush Structure"))
  (return true "NewEnumerator2" false "Open cell"))

(fn `UserConstructionScript`
  (`parent.UserConstructionScript`))