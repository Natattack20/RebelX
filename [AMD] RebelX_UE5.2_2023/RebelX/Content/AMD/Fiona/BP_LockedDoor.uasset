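; BP_LockedDoor is an interactable door that opens only when the Player_RebelX character holds a cell key.
; GetInteractionType supplies the prompt, and ActivateSceneObject checks the HasCellKey flag on the player reference cached at BeginPlay.
; With the key, a Timeline lerps the door's yaw to swing it open, then clears the flag on finish.
; Without it, a UI_NeedKey widget is added to the viewport.
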(event `self.ReceiveBeginPlay`
  (bind _asplayer_rebel_x (cast `/Game/RebelX_Core/Blueprints/Player_RebelX` (`GameplayStatics.GetPlayerCharacter` 0)))
  (set `self.As Player Rebel X` _asplayer_rebel_x))

(event `/Game/RebelX_Core/Blueprints/Interfaces/BPI_Interactables.ActivateSceneObject`
  (bind (_door_rotation_roll _door_rotation_pitch _door_rotation_yaw) (`KismetMathLibrary.BreakRotator` (`self.door rotation`)))
  (if (`/Game/RebelX_Core/Blueprints/Player_RebelX.HasCellKey` (`self.As Player Rebel X`))
    (set `self.door rotation` (`self.K2_GetActorRotation`))
    (bind (_direction _newtrack_0) (`Timeline|Timeline` :!via `PlayFromStart`)
      (:`Update`
        (`self.K2_SetActorRelativeRotation` (`KismetMathLibrary.MakeRotator` _door_rotation_roll _door_rotation_pitch (`KismetMathLibrary.Lerp` _door_rotation_yaw (- _door_rotation_yaw 80.0) _newtrack_0))))
      (:`Finished`
        (set `/Game/RebelX_Core/Blueprints/Player_RebelX.HasCellKey` false (`self.As Player Rebel X`))))
    (else
      (bind _returnvalue (`|CreateWidget` "/Game/AMD/Fiona/UI_NeedKey.UI_NeedKey_C"))
      (`UserWidget.AddToViewport` _returnvalue 0))))

(fn `GetInteractionType`
  (returns (`Return Value` :type Boolean) (InteractionType :type "/Game/RebelX_Core/Blueprints/Enums/E_InteractionTyoes Enum") (Consumeable :type Boolean) (InteractionMessage :type Text) (IconBrush :type "SlateBrush Structure"))
  (return false "NewEnumerator2" false "       E to \nOpen Door?"))

(fn `UserConstructionScript`
  (`parent.UserConstructionScript`))