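; BP_LockedDoorPin is an interactable locked door that offers an "Open Door?" prompt and uses a PIN entry widget.
; Activating it toggles the UI_WeaponPin widget until Completed is set, restoring game-only input and hiding the cursor on close.
; A separate OpenDoor event, not called within this graph, swings the door's yaw 80 degrees through a Timeline-driven Lerp.
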(event `self.ReceiveBeginPlay`
  (bind _asplayer_rebel_x (cast `/Game/RebelX_Core/Blueprints/Player_RebelX` (`GameplayStatics.GetPlayerCharacter` 0)))
  (set `self.As Player Rebel X` _asplayer_rebel_x))

(event `OpenDoor`
  (bind (_door_rotation_roll _door_rotation_pitch _door_rotation_yaw) (`KismetMathLibrary.BreakRotator` (`self.door rotation`)))
  (set `self.door rotation` (`self.K2_GetActorRotation`))
  (bind (_direction _newtrack_0) (`Timeline|Timeline` :!via `PlayFromStart`)
    (:`Update`
      (`self.K2_SetActorRelativeRotation` (`KismetMathLibrary.MakeRotator` _door_rotation_roll _door_rotation_pitch (`KismetMathLibrary.Lerp` _door_rotation_yaw (- _door_rotation_yaw 80.0) _newtrack_0))))))

(event `/Game/RebelX_Core/Blueprints/Interfaces/BPI_Interactables.ActivateSceneObject`
  (bind _returnvalue (`GameplayStatics.GetPlayerController` 0))
  (if (`self.Completed`)
    _
    (elif (`self.Open`)
      (`WidgetBlueprintLibrary.SetInputMode_GameOnly` _returnvalue)
      (set `PlayerController.bShowMouseCursor` false _returnvalue)
      (set `self.Open` false)
      (`Widget.RemoveFromParent` (stale _returnvalue_2))
      (else
        (set `self.Open` true)
        (bind _returnvalue_2 (`|CreateWidget` "/Game/AMD/Fiona/UI_WeaponPin.UI_WeaponPin_C" null self))
        (`UserWidget.AddToViewport` _returnvalue_2 0)))))

(fn `GetInteractionType`
  (returns (`Return Value` :type Boolean) (InteractionType :type "/Game/RebelX_Core/Blueprints/Enums/E_InteractionTyoes Enum") (Consumeable :type Boolean) (InteractionMessage :type Text) (IconBrush :type "SlateBrush Structure"))
  (return false "NewEnumerator2" false "Open Door?"))

(fn `UserConstructionScript`
  (`parent.UserConstructionScript`))