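; Broken canteen light actor with two rect lights that can flicker during play.
; The construction script sets both lights to the Intensity variable.
; On BeginPlay, if Flicker is set, the Flickering timeline drives both between zero and double that intensity.
; A FlipFlop on the timeline's Finished output alternates reverse and forward playback to keep the flicker looping.
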(event `self.ReceiveBeginPlay`
  (if (`self.Flicker?`)
    (bind (_direction _newtrack_0) (`Timeline|Flickering` :!via `PlayFromStart` :!label _label)
      (:`Update`
        (`LightComponent.SetIntensity` (`self.RectLight`) (`KismetMathLibrary.Lerp` 0.0 (* (`self.Intensity`) 2.0) _newtrack_0))
        (`LightComponent.SetIntensity` (`self.RectLight1`) (`KismetMathLibrary.Lerp` 0.0 (* (`self.Intensity`) 2.0) _newtrack_0)))
      (:`Finished`
        (`/Engine/EditorBlueprintResources/StandardMacros.FlipFlop`
          (:`A`
            (goto _label :!via `ReverseFromEnd`))
          (:`B`
            (goto _label :!via `PlayFromStart`)))))))

(fn `UserConstructionScript`
  (`LightComponent.SetIntensity` (`self.RectLight`) (`self.Intensity`))
  (`LightComponent.SetIntensity` (`self.RectLight1`) (`self.Intensity`)))