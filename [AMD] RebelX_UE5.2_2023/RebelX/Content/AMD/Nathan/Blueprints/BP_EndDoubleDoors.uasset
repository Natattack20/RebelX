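; End-of-level double doors that let Player_RebelX travel to the P_Yard+Lighting level.
; Overlapping EndDoorBox shows the EtoOpen prompt and grants access; pressing E while not closed stores the player in the game instance, then loads the level after a short delay.
; CloseDoor and OpenDoor set the lock flag and show or hide six collisionless meshes.
; The construction script poses the right door ajar when Open is set.
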(event `self.ReceiveBeginPlay`
  (`PrimitiveComponent.SetCollisionEnabled` (`self.StaticMesh`) "NoCollision")
  (`PrimitiveComponent.SetCollisionEnabled` (`self.StaticMesh2`) "NoCollision")
  (`PrimitiveComponent.SetCollisionEnabled` (`self.StaticMesh3`) "NoCollision")
  (`PrimitiveComponent.SetCollisionEnabled` (`self.StaticMesh4`) "NoCollision")
  (`PrimitiveComponent.SetCollisionEnabled` (`self.StaticMesh1`) "NoCollision")
  (`PrimitiveComponent.SetCollisionEnabled` (`self.StaticMesh5`) "NoCollision"))

(event `self.EndDoorBox.OnComponentBeginOverlap`
  (params (OverlappedComponent :type "PrimitiveComponent Object Reference") (OtherActor :type "Actor Object Reference") (OtherComp :type "PrimitiveComponent Object Reference") (OtherBodyIndex :type Integer) (bFromSweep :type Boolean) (SweepResult :type "HitResult Structure (by ref)"))
  (cast `/Game/RebelX_Core/Blueprints/Player_RebelX` OtherActor)
  (`self.EnableInput` (`GameplayStatics.GetPlayerController` 0))
  (set `self.Access?` true)
  (bind _returnvalue (`|CreateWidget` "/Game/AMD/Nathan/Widgets/E-to-Open.E-to-Open_C"))
  (`UserWidget.AddToViewport` _returnvalue 0))

(event `self.EndDoorBox.OnComponentEndOverlap`
  (params (OverlappedComponent :type "PrimitiveComponent Object Reference") (OtherActor :type "Actor Object Reference") (OtherComp :type "PrimitiveComponent Object Reference") (OtherBodyIndex :type Integer))
  (cast `/Game/RebelX_Core/Blueprints/Player_RebelX` OtherActor)
  (`self.EnableInput` (`GameplayStatics.GetPlayerController` 0))
  (set `self.Access?` false)
  (`Widget.RemoveFromParent` (stale `self.EndDoorBox.OnComponentBeginOverlap` _returnvalue)))

(event `Key|E`
  (params (Key :type "Key Structure"))
  (:`Pressed`
    (if (and (`self.Access?`) (not (`self.Closed`)))
      (`/Game/AMD/Instance.Store Player` (cast `/Game/AMD/Instance` (`GameplayStatics.GetGameInstance`) :!pure true))
      (`KismetSystemLibrary.Delay` 0.2)
      (`GameplayStatics.OpenLevel` "P_Yard+Lighting"))))

(event `Close Door`
  (set `self.Closed` true)
  (`SceneComponent.SetVisibility` (`self.StaticMesh`) true false)
  (`SceneComponent.SetVisibility` (`self.StaticMesh2`) true false)
  (`SceneComponent.SetVisibility` (`self.StaticMesh3`) true false)
  (`SceneComponent.SetVisibility` (`self.StaticMesh4`) true false)
  (`SceneComponent.SetVisibility` (`self.StaticMesh1`) true false)
  (`SceneComponent.SetVisibility` (`self.StaticMesh5`) true false))

(event `Open Door`
  (set `self.Closed` false)
  (`SceneComponent.SetVisibility` (`self.StaticMesh`) false false)
  (`SceneComponent.SetVisibility` (`self.StaticMesh2`) false false)
  (`SceneComponent.SetVisibility` (`self.StaticMesh3`) false false)
  (`SceneComponent.SetVisibility` (`self.StaticMesh4`) false false)
  (`SceneComponent.SetVisibility` (`self.StaticMesh1`) false false)
  (`SceneComponent.SetVisibility` (`self.StaticMesh5`) false false))

(fn `UserConstructionScript`
  (if (`self.Open?`)
    (`|ExecutionSequence`
      (:`then_0`
        (`SceneComponent.K2_SetRelativeLocationAndRotation` (`self.Right Door`) (120.0 -40.0 0.0) (struct :`Yaw` 130.0) false false)))))