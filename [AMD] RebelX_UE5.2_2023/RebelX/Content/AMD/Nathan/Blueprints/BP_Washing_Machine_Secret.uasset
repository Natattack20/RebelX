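; BP_Washing_Machine_Secret is an interactable secret washing machine whose door the player can open.
; A Box overlap with Player_RebelX enables input and sets an Access flag, and leaving the box reverses both.
; Pressing E plays the OpenSesame timeline to rotate the door up to 90 degrees, then sets Opened so it cannot be triggered again.
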(event `self.Box.OnComponentBeginOverlap`
  (params (OverlappedComponent :type "PrimitiveComponent Object Reference") (OtherActor :type "Actor Object Reference") (OtherComp :type "PrimitiveComponent Object Reference") (OtherBodyIndex :type Integer) (bFromSweep :type Boolean) (SweepResult :type "HitResult Structure (by ref)"))
  (cast `/Game/RebelX_Core/Blueprints/Player_RebelX` OtherActor)
  (`self.EnableInput` (`GameplayStatics.GetPlayerController` 0))
  (set `self.Access` true))

(event `self.Box.OnComponentEndOverlap`
  (params (OverlappedComponent :type "PrimitiveComponent Object Reference") (OtherActor :type "Actor Object Reference") (OtherComp :type "PrimitiveComponent Object Reference") (OtherBodyIndex :type Integer))
  (cast `/Game/RebelX_Core/Blueprints/Player_RebelX` OtherActor)
  (`self.DisableInput` (`GameplayStatics.GetPlayerController` 0))
  (set `self.Access` false))

(event `Key|E` :consume false
  (params (Key :type "Key Structure"))
  (:`Pressed`
    (if (and (not (`self.Opened`)) (`self.Access`))
      (bind (_direction _washing_door_rotation) (`Timeline|Open Sesame` :!via `PlayFromStart`)
        (:`Update`
          (`SceneComponent.K2_SetRelativeRotation` (`self.Washing Machine Door`) (`KismetMathLibrary.RLerp` (struct) (struct :`Yaw` 90.0) _washing_door_rotation) false false))
        (:`Finished`
          (set `self.Opened` true))))))

(fn `UserConstructionScript`)