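; Key pickup actor that Player_RebelX collects by pressing E while standing inside its Box trigger.
; Box overlap toggles input, the Access flag and the E prompt's visibility, and Tick yaws the prompt toward the player's capsule.
; Pressing E sets Collected, hides key and prompt, and plays a pickup sound.
; The actor is never destroyed and Collected is never checked here, so re-entering shows the prompt again.
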(event `self.ReceiveTick`
  (params (DeltaSeconds :type "Float (single-precision)"))
  (bind (_returnvalue_roll _returnvalue_pitch _returnvalue_yaw) (`KismetMathLibrary.BreakRotator` (`KismetMathLibrary.FindLookAtRotation` (`SceneComponent.K2_GetComponentLocation` (`self.E`)) (`SceneComponent.K2_GetComponentLocation` (`Character.CapsuleComponent` (cast `/Game/RebelX_Core/Blueprints/Player_RebelX` (`GameplayStatics.GetPlayerCharacter` 0) :!pure true))))))
  (`SceneComponent.K2_SetWorldRotation` (`self.E`) (`KismetMathLibrary.MakeRotator` 0.0 0.0 _returnvalue_yaw) false false))

(event `self.Box.OnComponentBeginOverlap`
  (params (OverlappedComponent :type "PrimitiveComponent Object Reference") (OtherActor :type "Actor Object Reference") (OtherComp :type "PrimitiveComponent Object Reference") (OtherBodyIndex :type Integer) (bFromSweep :type Boolean) (SweepResult :type "HitResult Structure (by ref)"))
  (cast `/Game/RebelX_Core/Blueprints/Player_RebelX` OtherActor)
  (`self.EnableInput` (`GameplayStatics.GetPlayerController` 0))
  (`SceneComponent.SetVisibility` (`self.E`) true false)
  (set `self.Access` true))

(event `self.Box.OnComponentEndOverlap`
  (params (OverlappedComponent :type "PrimitiveComponent Object Reference") (OtherActor :type "Actor Object Reference") (OtherComp :type "PrimitiveComponent Object Reference") (OtherBodyIndex :type Integer))
  (cast `/Game/RebelX_Core/Blueprints/Player_RebelX` OtherActor)
  (`self.DisableInput` (`GameplayStatics.GetPlayerController` 0))
  (`SceneComponent.SetVisibility` (`self.E`) false false)
  (set `self.Access` false))

(event `Key|E` :consume false
  (params (Key :type "Key Structure"))
  (:`Pressed`
    (if (`self.Access`)
      (set `self.Collected` true)
      (`SceneComponent.SetVisibility` (`self.Key`) false false)
      (`SceneComponent.SetVisibility` (`self.E`) false false)
      (`GameplayStatics.PlaySoundAtLocation` "/Game/RebelX_Core/Audio/Weapon/SC_Pickup_Ammo.SC_Pickup_Ammo" (`self.K2_GetActorLocation`) (struct) 1.0 1.0 0.0 null null null null))))

(fn `UserConstructionScript`)