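; Double door actor that the Player_RebelX character unlocks with a collected key.
; Its trigger box toggles input and shows an EtoOpen prompt while locked; pressing E inside opens it if any assigned Key is collected.
; OpenDoor plays a sound and runs the OpenSesame timeline to lerp both leaves; CloseDoor reverses it but is not called here.
; The Open flag poses the doors open in the construction script.
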(event `Key|E` :consume false
  (params (Key :type "Key Structure"))
  (:`Pressed`
    (`KismetSystemLibrary.PrintString` "Hello")
    (if (and (not (`self.Key Found`)) (`self.Key?`) (`self.Access?`))
      (for _array_element (`self.Key`)
        (if (`/Game/AMD/Nathan/Blueprints/BP_Key.Collected` _array_element)
          (`/Engine/EditorBlueprintResources/StandardMacros.DoOnce` false
            (:`Completed`
              (set `self.Key Found` true)
              (`self.Open Door`)
              (`Widget.RemoveFromParent` (stale `self.Box.OnComponentBeginOverlap` _returnvalue_2)))))))))

(event `Open Door`
  (`GameplayStatics.PlaySoundAtLocation` "/Game/AMD/Nathan/Audio/Prison_Door_Opening.Prison_Door_Opening" (`SceneComponent.K2_GetComponentLocation` (`self.DefaultSceneRoot`)) (struct) 1.0 1.0 0.0 null null null null)
  (bind (_direction _open) (`Timeline|Open Sesame` :!via `PlayFromStart` :!label _label)
    (:`Update`
      (`SceneComponent.K2_SetRelativeLocationAndRotation` (`self.Left Door`) (`KismetMathLibrary.VLerp` (-60.0 0.0 0.0) (`self.Left Door Vector`) _open) (`KismetMathLibrary.RLerp` (struct) (struct :`Yaw` 50.0) _open) false false)
      (`SceneComponent.K2_SetRelativeLocationAndRotation` (`self.Right Door`) (`KismetMathLibrary.VLerp` (40.0 0.0 0.0) (`self.Right Door Vector`) _open) (`KismetMathLibrary.RLerp` (struct) (struct :`Yaw` -50.0) _open) false false))))

(event `Close Door`
  (goto _label :!via `ReverseFromEnd`))

(event `self.Box.OnComponentBeginOverlap`
  (params (OverlappedComponent :type "PrimitiveComponent Object Reference") (OtherActor :type "Actor Object Reference") (OtherComp :type "PrimitiveComponent Object Reference") (OtherBodyIndex :type Integer) (bFromSweep :type Boolean) (SweepResult :type "HitResult Structure (by ref)"))
  (bind _returnvalue (`GameplayStatics.GetPlayerController` 0))
  (cast `/Game/RebelX_Core/Blueprints/Player_RebelX` OtherActor)
  (`self.EnableInput` _returnvalue)
  (set `self.Access?` true)
  (if (and (not (`self.Key Found`)) (`self.Key?`))
    (bind _returnvalue_2 (`|CreateWidget` "/Game/AMD/Nathan/Widgets/E-to-Open.E-to-Open_C" _returnvalue))
    (`UserWidget.AddToViewport` _returnvalue_2 0)))

(event `self.Box.OnComponentEndOverlap`
  (params (OverlappedComponent :type "PrimitiveComponent Object Reference") (OtherActor :type "Actor Object Reference") (OtherComp :type "PrimitiveComponent Object Reference") (OtherBodyIndex :type Integer))
  (cast `/Game/RebelX_Core/Blueprints/Player_RebelX` OtherActor)
  (`self.DisableInput` (`GameplayStatics.GetPlayerController` 0))
  (set `self.Access?` false)
  (if (and (not (`self.Key Found`)) (`self.Key?`))
    (`Widget.RemoveFromParent` (stale `self.Box.OnComponentBeginOverlap` _returnvalue_2))))

(fn `UserConstructionScript`
  (if (`self.Open?`)
    (`|ExecutionSequence`
      (:`then_0`
        (`SceneComponent.K2_SetRelativeLocationAndRotation` (`self.Right Door`) (120.0 -40.0 0.0) (struct :`Yaw` 130.0) false false))
      (:`then_1`
        (`SceneComponent.K2_SetRelativeLocationAndRotation` (`self.Left Door`) (-140.0 -40.0 0.0) (struct :`Yaw` 50.0) false false)))))