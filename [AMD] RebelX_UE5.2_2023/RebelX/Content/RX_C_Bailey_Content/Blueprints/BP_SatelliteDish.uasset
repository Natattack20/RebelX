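; BP_SatelliteDish is a destructible satellite dish that only takes damage instigated by the first player's controller.
; AnyDamage passes through a Gate, lowers clamped Health and shows a hit marker on the RebelX HUD.
; At zero Health it closes the Gate against further damage, kills its light, plays explosion effects and audio, and launches the mesh upward with physics.
; It then calls SatelliteDestroyed to signal the destruction.
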(event `Stop Damage`
  (goto _label :!via `Close`))

(event `self.ReceiveAnyDamage`
  (params (Damage :type "Float (single-precision)") (DamageType :type "DamageType Object Reference") (InstigatedBy :type "Controller Object Reference") (DamageCauser :type "Actor Object Reference"))
  (`/Engine/EditorBlueprintResources/StandardMacros.Gate` false :!label _label
    (:`Exit`
      (if (== InstigatedBy (`GameplayStatics.GetPlayerController` 0))
        (bind _output_get (set `self.Health` (`KismetMathLibrary.FClamp` (- (`self.Health`) Damage) 0.0 1000.0)))
        (`|ExecutionSequence`
          (:`then_0`
            ;[1 1 1] Hit Marker
            (message `/Game/RebelX_Core/Blueprints/Interfaces/BPI_HUD.ShowHitMark` (cast `/Game/RebelX_Core/Blueprints/HUD_RebelX` (`PlayerController.GetHUD` (`Pawn.GetLocalViewingPlayerController` (`GameplayStatics.GetPlayerCharacter` 0))) :!pure true)))
          (:`then_1`
            (if (<= _output_get 0.0)
              (`|ExecutionSequence`
                (:`then_0`
                  (`self.Stop Damage`))
                (:`then_1`
                  ;[1 1 1] Visual/Aduio Feedback
                  (`LightComponent.SetIntensity` (`self.PointLight`) 0.0)
                  (`ActorComponent.Activate` (`self.Explosion`) false)
                  (`AudioComponent.Play` (`self.Audio_Explosion`) 0.0)
                  (`PrimitiveComponent.SetSimulatePhysics` (`self.SM_SatDish`) true)
                  (`PrimitiveComponent.AddImpulse` (`self.SM_SatDish`) (0.0 0.0 100000.0) "None" false))
                (:`then_2`
                  (`self.Satellite Destroyed`))))))))))

(fn `UserConstructionScript`
  (`parent.UserConstructionScript`))